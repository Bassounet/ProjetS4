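; BP_Lights_Du_Bled drives the horror main menu scene, creating WBP_Menu on BeginPlay and looping a flickering light sequence with mannequins.
; A timeline replayed over seven counted steps toggles its rect lights and BP_LightBlinkMenu's point light, using track thresholds to show, hide and teleport BP_Menu_StepMannikin's mannequins.
; The last step warms the light temperature, shakes the camera and raises the AnimScreamer flag before the cycle restarts.
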(event Custom|BlinkerStep
  (bind _blinker_1 (Timeline|Timeline_Step PlayFromStart)
    (:Update
      (bind _returnvalue (Actor|GetActorOfClass "/Game/Level/Antoine/BP_LightBlinkMenu.BP_LightBlinkMenu_C"))
      (if (and (<= (Variables|Default|GetStep) 2.0) (>= (Variables|Default|GetStep) 1.0))
        (Rendering|SetVisibility (Variables|Default|GetRectLight) (>= _blinker_1 1.0) false)
        (else
          (Rendering|SetVisibility (Variables|Default|GetRectLightComponent) (>= _blinker_1 1.0) false)
          (Rendering|SetVisibility (Variables|/Game/Level/Antoine/BP_LightBlinkMenu.BP_LightBlinkMenu_C|GetPointLight _returnvalue) false false)))
      (bind _returnvalue_2 (Actor|GetActorOfClass "/Game/Level/Antoine/BP_Menu_StepMannikin.BP_Menu_StepMannikin_C"))
      (CallFunction|SpawnMannikin)
      (CallFunction|VerifTemperatureLights)
      (CallFunction|VerifAnimScreamer)
      (if (>= _blinker_1 1.5)
        (Default|ShowMannikins _returnvalue_2)
        (else
          (Default|HideMannikins _returnvalue_2))))
    (:Finished
      (bind _output_get (Variables|Default|SetStep (+ (Variables|Default|GetStep) 1.0)))
      (if (< _output_get 7.0)
        (Utilities|FlowControl|Delay 6.0)
        (Timeline|Timeline_Step PlayFromStart)
        (else
          (Variables|Default|SetStep 0.0)
          (Utilities|FlowControl|Delay 1.0)
          (Timeline|Timeline_Step PlayFromStart))))))

(event Custom|Spawn%20Mannikin
  (if (or (>= (stale Custom|BlinkerStep _blinker_1) 2.0) (<= (stale Custom|BlinkerStep _blinker_1) -1.0))
    (bind _returnvalue (Actor|GetActorOfClass "/Game/Level/Antoine/BP_Menu_StepMannikin.BP_Menu_StepMannikin_C"))
    (Default|MannikinsTeleport _returnvalue)))

(event Custom|Verif%20Temperature%20Lights
  (bind _returnvalue (Actor|GetActorOfClass "/Game/Level/Antoine/BP_LightBlinkMenu.BP_LightBlinkMenu_C"))
  (if (== (Variables|Default|GetStep) 6.0)
    (Utilities|FlowControl|Delay 0.7)
    (Class|LightComponent|SetTemperature (Variables|Default|GetRectLight) 5e+02)
    (else
      (Utilities|FlowControl|Delay 0.7)
      (Class|LightComponent|SetTemperature (Variables|Default|GetRectLightComponent) 6.5e+03))))

(event Custom|Verif%20Anim%20Screamer
  (if (== (Variables|Default|GetStep) 6.0)
    (Utilities|FlowControl|Delay 1.2)
    (CameraShakes|StartCameraShake (Game|GetPlayerCameraManager 0) "/Script/Engine.CameraShakeBase" 1.0 "World" "0, 0, 0")
    (Variables|Default|SetAnim%20Screamer true)
    (else
      (Variables|Default|SetAnim%20Screamer false))))

(event Custom|Widget%20Caller
  (bind _returnvalue (UserInterface|CreateWidget "/Game/Level/Antoine/WBP_Menu.WBP_Menu_C"))
  (bind _output_get (Variables|Default|SetMain%20Menu _returnvalue))
  (UserInterface|Viewport|AddtoViewport _output_get 0)
  (Input|SetInputModeUIOnly (Game|GetPlayerController 0) (Variables|/Game/Level/Antoine/WBP_Menu.WBP_Menu_C|GetButton_NewGame _returnvalue) "DoNotLock"))

(event EventBeginPlay
  (CallFunction|WidgetCaller)
  (Utilities|FlowControl|Delay 2.0)
  (CallFunction|BlinkerStep))

(fn ConstructionScript)