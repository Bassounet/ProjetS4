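; Mannequin actor for the menu that starts hidden at the world origin and repositions as the step held by BP_Lights_Du_Bled changes.
; Mannikinsteleport reads that step and uses it to index per-step location and rotation arrays for an instant teleport.
; The same event shows both eye components only on step six.
; Separate show and hide events toggle the skeletal mesh without affecting its children.
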(event Custom|Mannikins%20teleport
  (bind _returnvalue (Actor|GetActorOfClass "/Game/Level/Antoine/BP_Lights_Du_Bled.BP_Lights_Du_Bled_C"))
  (Transformation|SetActorLocationAndRotation (Components|GetOwner (Variables|Default|GetSkeletalMesh)) (Utilities|Array|Get(acopy) (Variables|Default|GetLocation_Step) (Math|Float|Truncate (Variables|/Game/Level/Antoine/BP_Lights_Du_Bled.BP_Lights_Du_Bled_C|GetStep _returnvalue))) (Utilities|Array|Get(acopy) (Variables|Default|GetRotation%20Step) (Math|Float|Truncate (Variables|/Game/Level/Antoine/BP_Lights_Du_Bled.BP_Lights_Du_Bled_C|GetStep _returnvalue))) false true)
  (Rendering|SetVisibility (Variables|Default|GetEye_R) (== (Variables|/Game/Level/Antoine/BP_Lights_Du_Bled.BP_Lights_Du_Bled_C|GetStep _returnvalue) 6.0) true))

(event Custom|Show%20Mannikins
  (Rendering|SetVisibility (Variables|Default|GetSkeletalMesh) true false))

(event Custom|Hide%20Mannikins
  (Rendering|SetVisibility (Variables|Default|GetSkeletalMesh) false false))

(event EventBeginPlay
  (Rendering|SetVisibility (Variables|Default|GetSkeletalMesh) false true)
  (Transformation|SetActorLocationAndRotation "0, 0, 0" "0, 0, 0" false true))

(fn ConstructionScript)