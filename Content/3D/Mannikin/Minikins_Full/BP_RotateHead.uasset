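; Actor Blueprint for a Minikins mannequin that tracks the player with a look-at rotation, named for head rotation.
; BeginPlay caches the player character.
; While CanRotate is set, Tick stores the look-at rotation from the skeletal mesh's world location to the player in TargetRotation.
; The graph only computes this value and does not apply it to the mesh or a bone.
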(event EventBeginPlay
  (Variables|Default|SetPlayerRef (Game|GetPlayerCharacter 0)))

(event EventTick
  (params (DeltaSeconds :type Float%20%28single-precision%29))
  (if (Variables|Default|GetCanRotate)
    (Variables|Default|SetTargetRotation (Math|Rotator|FindLookatRotation (Transformation|GetWorldLocation (Variables|Default|GetSkeletalMesh)) (Transformation|GetActorLocation (Variables|Default|GetPlayerRef))))))

(fn ConstructionScript)