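; BP_GI, apparently the Game Instance, stores player options: voice gender, keyboard or gamepad choice, X and Y rotation inversion, and four volume levels.
; Simple setters write each option.
; SetSoundMix saves the Master, Music, SFX and Voice volumes, then applies each through a sound class override and pushes its matching mix modifier.
; GetSoundMixVar returns the saved volumes.
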(fn MaleFemaleVoice
  (params (MaleFemale :type EN_MaleFemaleVoice%20Enum :default "NewEnumerator0"))
  (Variables|Default|SetMaleFemale MaleFemale))

(fn ClavierManette
  (params (ManetteClavier :type EN_ClavierManette%20Enum :default "NewEnumerator0"))
  (Variables|Default|SetManetteClavier ManetteClavier))

(fn SetXRotate
  (params (Invertx? :type Boolean))
  (Variables|Default|SetInvertx? Invertx?))

(fn SetYRotate
  (params (Inverty? :type Boolean))
  (Variables|Default|SetInverty? Inverty?))

(fn SetSoundMix
  (params (VolumeSFX :type Float%20%28single-precision%29) (VolumeMUSIC :type Float%20%28single-precision%29) (VolumeMASTER :type Float%20%28single-precision%29) (VolumeVOICE :type Float%20%28single-precision%29))
  (bind _output_get (Variables|Default|SetVolume%20SFX VolumeSFX))
  (bind _output_get_2 (Variables|Default|SetVolume%20MUSIC VolumeMUSIC))
  (bind _output_get_3 (Variables|Default|SetVolume%20MASTER VolumeMASTER))
  (bind _output_get_4 (Variables|Default|SetVolume%20VOICE VolumeVOICE))
  (Audio|SetSoundMixClassOverride "/Game/SND/SCM_SFX.SCM_SFX" "/Game/SND/SFX.SFX" _output_get 1.0 0.0 true)
  (Audio|PushSoundMixModifier "/Game/SND/SCM_SFX.SCM_SFX")
  (Audio|SetSoundMixClassOverride "/Game/SND/SCM_Music.SCM_Music" "/Game/SND/Music.Music" _output_get_2 1.0 0.0 true)
  (Audio|PushSoundMixModifier "/Game/SND/SCM_Music.SCM_Music")
  (Audio|SetSoundMixClassOverride "/Game/SND/SCM_Master.SCM_Master" "/Game/SND/Master.Master" _output_get_3 1.0 0.0 true)
  (Audio|PushSoundMixModifier "/Game/SND/SCM_Master.SCM_Master")
  (Audio|SetSoundMixClassOverride "/Game/SND/SCM_Voices.SCM_Voices" "/Game/SND/Voice.Voice" _output_get_4 1.0 0.0 true)
  (Audio|PushSoundMixModifier "/Game/SND/SCM_Voices.SCM_Voices"))

(fn GetSoundMixVar
  (return (Variables|Default|GetVolume%20MASTER) (Variables|Default|GetVolume%20MUSIC) (Variables|Default|GetVolume%20SFX) (Variables|Default|GetVolume%20VOICE)))