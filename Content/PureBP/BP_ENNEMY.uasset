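; Enemy pawn Blueprint that hands its behavior tree to a My_AIC controller on BeginPlay.
; Pawn Sensing sets SeePlayer to true on spotting a FirstPersonCharacter, and this file never resets it.
; Ronde (looping random patrol around StartingLocation at walk speed) and Chase (run to the player, then print a debug string) are custom events marked as an old version and not called here.
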(event OnSeePawn(PawnSensing)
  (params (Pawn :type Pawn%20Object%20Reference))
  ;[0 1 0.01909] SeeingPlayer
  (Utilities|Casting|CastToFirstPersonCharacter Pawn)
  (Variables|Default|SetSeePlayer true))

(event Custom|Chase
  ;[1 0 0.1472] OLD VERSION
  ;;[1 1 1] Ronde
  (Variables|/Script/Engine.CharacterMovementComponent|SetMaxWalkSpeed (Variables|Character|GetCharacterMovement) (Variables|Default|GetRun_Speed))
  (AI|AIMoveTo self "0, 0, 0" (Game|GetPlayerCharacter 0) 5.0 false
    (:OnSuccess
      (Utilities|FlowControl|RetriggerableDelay (Math|Random|RandomFloatinRange 0.5 1.0))
      (Development|PrintString "JteBute"))))

(event Custom|Ronde
  ;[1 0 0.1472] OLD VERSION
  ;;[1 1 1] Ronde
  (Variables|/Script/Engine.CharacterMovementComponent|SetMaxWalkSpeed (Variables|Character|GetCharacterMovement) (Variables|Default|GetWalk_Speed))
  (AI|AIMoveTo self (.RandomLocation (AI|Navigation|GetRandomReachablePointinRadius (Variables|Default|GetStartingLocation) (Variables|Default|GetRadius_Ronde) 0 0)) 0 5.0 false
    (:OnSuccess
      (Utilities|FlowControl|RetriggerableDelay (Math|Random|RandomFloatinRange 0.5 1.0))
      (CallFunction|Ronde))))

(event EventBeginPlay
  ;[0 0.1828 1] Start
  (bind _asmy_aic (Utilities|Casting|CastToMy_AIC (AI|GetAIController self)))
  (Default|SetupAIC _asmy_aic (Variables|Default|GetBTAsset)))

(fn ConstructionScript)