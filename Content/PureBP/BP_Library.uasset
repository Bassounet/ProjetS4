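; BP_Library is a collection of shared helper functions for camera shakes and access to common game objects.
; Loud and light shakes play as world camera shakes, the loud one at a given epicenter and the light one at the player's location.
; Getters return the cast FirstPersonCharacter, its main HUD reference, and the BP_GI game instance through RecupDispatcherDie.
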(fn CamShakeLoud
  (params (Epicenter :type Vector))
  (Camera|PlayWorldCameraShake 0 "/Game/PureBP/Feedback/BP_CamShakeLoud.BP_CamShakeLoud_C" Epicenter 5e+02))

(fn CamShakeLight
  (Camera|PlayWorldCameraShake 0 "/Game/PureBP/Feedback/BP_CamShakeLight.BP_CamShakeLight_C" (Transformation|GetActorLocation (Game|GetPlayerCharacter 0)) 5e+02))

(fn RecupDispatcherDie
  (bind _asbp_gi (Utilities|Casting|CastToBP_GI (Game|GetGameInstance)))
  (return _asbp_gi))

(fn GetHUD
  (bind _asfirst_person_character (CallFunction|GetPlayer))
  (return (Variables|/Game/PureBP/FirstPersonCharacter.FirstPersonCharacter_C|GetREF_MainHud _asfirst_person_character)))

(fn GetPlayer
  (bind _asfirst_person_character (Utilities|Casting|CastToFirstPersonCharacter (Game|GetPlayerCharacter 0)))
  (return _asfirst_person_character))