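; BP_MenuController is the player controller for the main menu, which it creates and adds to the viewport on BeginPlay.
; It uses Game and UI input with focus on the New Game button, a locked mouse and a visible cursor.
; Any key press records whether a gamepad is in use through UsingGamepad.
; An unconnected UI-only input mode node remains in the graph.
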(event EventBeginPlay
  (bind _returnvalue (UserInterface|CreateWidget "/Game/PureBP/UI/BP/WBP_Menu.WBP_Menu_C" 0 self))
  (bind _output_get (Variables|Default|SetMain%20Menu _returnvalue))
  (UserInterface|Viewport|AddtoViewport _output_get 0)
  (Input|SetInputModeGameandUI self (Variables|/Game/PureBP/UI/BP/WBP_Menu.WBP_Menu_C|GetButton_NewGame _output_get) "LockAlways" true)
  (Variables|Default|SetbShowMouseCursor true))

(event EventTick
  (params (DeltaSeconds :type Float%20%28single-precision%29)))

(event Input|ActionEvents|InputActionMovingMenu
  (params (Key :type Key%20Structure :default "None")))

(event Input|KeyboardEvents|AnyKey
  (params (Key :type Key%20Structure :default "None"))
  (:Pressed
    (Variables|Default|SetUsingGamepad (Class|KismetInputLibrary|KeyIsGamepadKey Key))))

(fn ConstructionScript)