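; Enemy character, run by a My_AIC behavior tree with spline-built patrol points, that the player can blind and freeze with light.
; Looping timers accumulate exposure, moving it from smoke to flickering eyes to a time-dilation freeze.
; Retriggerable delays detect when light stops and clear the lit state, after a stun if fully blinded.
; Dispatchers pause movement during lore reading and cinematics; other events handle position reset and screen fade.
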(event Custom|BindForResetEverybody
  ;[1 1 1] Reset Location
  (EventDispatchers|BindEventtoResetAfterDie (Variables|Default|GetREF%20BP%20GI) (delegate Custom|ResetLocation)))

(event Custom|ResetLocation
  ;[1 1 1] Reset Location
  (Transformation|SetActorLocationAndRotation (Variables|REF|GetREF_Origin) "0, 0, 0"))

(event Custom|FixWhenReading
  ;[0 0.1828 1] Start
  (CallFunction|Pause))

(event Custom|UnFixAfterRead
  ;[0 0.1828 1] Start
  (CallFunction|UnPause))

(event Custom|Eye_On
  ;[0 1 0.03006] FeedBackLight
  ;;[1 1 1] Eye On
  (Rendering|SetVisibility (Variables|Default|GetL_Eye) true false))

(event Custom|OffEye
  ;[0 1 0.03006] FeedBackLight
  ;;[1 1 1] Eye Off
  (Utilities|Time|ClearandInvalidateTimerbyHandle (Variables|Default|GetREF_TimerClignotage))
  (Rendering|SetVisibility (Variables|Default|GetL_Eye) false false))

(event Custom|Freeze
  ;[0 1 0.03006] FeedBackLight
  ;;[1 1 1] Freeze Sound
  (if (not (Variables|Default|GetPlayed?))
    (Audio|PlaySoundatLocation "/Game/SND/Bank/Mannikins/SoundGreg/SC_EnnemyStun.SC_EnnemyStun" (Transformation|GetWorldLocation (Variables|Character|GetMesh)) "0, 0, 0" 5.0 1.0 0.0 "/Game/SND/SA_V1.SA_V1" 0 0 0)
    (Variables|Default|SetPlayed? true)
    (Variables|Default|SetCustomTimeDilation 0.0)))

(event Custom|BackFromLighting
  ;[0 1 0.03006] FeedBackLight
  ;;[1 1 1] Comment
  (CallFunction|Eyeon)
  (Audio|PlaySoundatLocation "/Game/SND/Bank/Mannikins/SoundGreg/SC_Revive.SC_Revive" (Transformation|GetWorldLocation (Variables|Character|GetMesh)) "0, 0, 0" 1.0 1.0 0.0 0 0 0 0)
  (Variables|Default|SetPlayed? false)
  (Variables|Default|SetCustomTimeDilation 1.0))

(event Custom|InteractSmoke
  (params (Activate? :type Boolean))
  (bind _ns_smokem (Variables|Default|GetNS_SmokeM))
  ;[1 1 1] Smoke FX
  (if Activate?
    (Components|Activation|Activate _ns_smokem false)
    (Variables|Default|SetNs_Activate? true)
    (else
      (Components|Activation|Deactivate _ns_smokem)
      (Variables|Default|SetNs_Activate? false))))

(event Custom|Pause
  ;[1 1 1] Comment
  (Components|Activation|Deactivate (Variables|Character|GetCharacterMovement))
  (EventDispatchers|UnbindallEventsfromPausewhenReadLore (Variables|Default|GetREF%20BP%20GI)))

(event Custom|Figer%20Ennemy
  ;[1 0.9448 0] Lighted
  ;;[1 1 1] Increment pour l'Aveugler
  (Default|Lighted (stale Custom|Lightedeuh _asmy_aic))
  (bind _output_get (Variables|Default|SetScoringLightStun (+ (Variables|Default|GetScoringLightStun) (Variables|Default|GetFrequance%20Increment%20point%20de%20light))))
  ;;;[1 1 1] Fige Complete
  (if (>= _output_get (Variables|Time|GetTime%20Exposition%20Before%20Stun%20After%20Blind))
    (Variables|Default|Setlighted true)
    (Variables|Default|SetCompleteBlind? true)
    (CallFunction|OffEye)
    (CallFunction|Freeze)))

(event Custom|UnPause
  ;[1 1 1] Comment
  (Components|Activation|Activate (Variables|Character|GetCharacterMovement) false)
  (EventDispatchers|UnbindallEventsfromUnPauseAfterRead (Variables|Default|GetREF%20BP%20GI)))

(event Custom|Clignogno
  ;[0 1 0.03006] FeedBackLight
  ;;[1 1 1] Clignotage Eye
  (Rendering|ToggleVisibility (Variables|Default|GetL_Eye) false))

(event Custom|FixCinematic
  ;[0 0.1828 1] Start
  (CallFunction|Pause))

(event Custom|UnFixCinematic
  ;[0 0.1828 1] Start
  (CallFunction|UnPause))

(event Custom|Lightedeuh
  ;[1 0.9448 0] Lighted
  (Variables|Default|Setlighted true)
  (bind _asmy_aic (Utilities|Casting|CastToMy_AIC (AI|GetAIController self)))
  (if (Variables|Default|GetRecentlyLighted?)
    (Utilities|FlowControl|Sequence
      (:then_0
        (if (Variables|Default|GetCompleteBlind?)
          ;;[1 1 1] Ennemy Delighté/ Défigé
          (Utilities|FlowControl|RetriggerableDelay (Variables|Time|GetTime%20Stun))
          (CallFunction|UnLightedeuh)
          (Variables|Default|SetRecentlyLighted? false)
          (Variables|Default|SetCompleteBlind? false)
          (Variables|Default|SetScoringLightStun 0.0)
          (Variables|Default|SetPlayerGrabbed? false)
          (else
            ;;[1 1 1] Un Lighté
            (Utilities|FlowControl|RetriggerableDelay 0.1)
            (if (not (Variables|Default|GetCompleteBlind?))
              (CallFunction|UnLightedeuh)
              (Variables|Default|SetRecentlyLighted? false)
              (Variables|Default|SetScoringLightStun 0.0)
              (CallFunction|Eyeon)))))
      (:then_1
        ;;[1 1 1] Direct après la light
        (Utilities|FlowControl|RetriggerableDelay 0.1)
        (Utilities|Time|ClearandInvalidateTimerbyHandle (Variables|REF|GetREF_TimerStun))
        (Utilities|Time|ClearandInvalidateTimerbyHandle (Variables|REF|GetREF_TimerWhenYouLightEnnemy))
        (Utilities|Time|ClearandInvalidateTimerbyHandle (Variables|Default|GetREF_TimerClignotage))
        (Variables|Default|SetScoringLight 0.0)
        (Variables|Default|SetRecentlyLighted? false)
        (Variables|Default|SetGoingStun? false)))
    (elif (not (Variables|Default|GetPlayerGrabbed?))
      ;;[1 1 1] Increment Pour le light
      (if (Variables|Default|GetNs_Activate?)
        _
        (else
          (CallFunction|InteractSmoke true)))
      (bind _returnvalue (Utilities|Time|SetTimerbyEvent (delegate Custom|CustomEvent_0) (Variables|Default|GetFrequance%20Increment%20point%20de%20light) true))
      (Variables|REF|SetREF_TimerWhenYouLightEnnemy _returnvalue)
      (Variables|Default|SetRecentlyLighted? true))))

(event Custom|CustomEvent_0
  ;[1 0.9448 0] Lighted
  ;;[1 1 1] Increment Pour le light
  (if (not (Variables|Default|GetGoingStun?))
    (Variables|Default|SetScoringLight (+ (Variables|Default|GetScoringLight) (Variables|Default|GetFrequance%20Increment%20point%20de%20light)))
    (if (> (Variables|Default|GetScoringLight) (Variables|Time|GetTemps%20Before%20Blind))
      (Variables|Default|Setlighted true)
      ;;[1 1 1] Increment pour l'Aveugler
      (CallFunction|Clignotage)
      (bind _returnvalue (Utilities|Time|SetTimerbyEvent (delegate Custom|Figer%20Ennemy) (Variables|Default|GetFrequance%20Increment%20point%20de%20light) true 0.1))
      (Variables|Default|SetRecentlyLighted? true)
      (Variables|Default|SetGoingStun? true)
      (Variables|REF|SetREF_TimerStun _returnvalue))))

(event Custom|UnLightedeuh
  ;[1 1 1] UnLight
  (Variables|Default|Setlighted false)
  (bind _asmy_aic (Utilities|Casting|CastToMy_AIC (AI|GetAIController self)))
  (Default|UnLighted _asmy_aic)
  (CallFunction|InteractSmoke false))

(event Custom|LaunchFade
  ;[1 1 1] Fade Laucnh
  (Default|FadeIN (Variables|REF|GetREF_Fade)))

(event Custom|Clignotage
  ;[0 1 0.03006] FeedBackLight
  ;;[1 1 1] Clignotage Eye
  (bind _returnvalue (Utilities|Time|SetTimerbyEvent (delegate Custom|Clignogno) (Math|Random|RandomFloatinRange 0.01 0.3) true))
  (Variables|Default|SetREF_TimerClignotage _returnvalue))

(event EventBeginPlay
  (bind _sphere3 (Variables|Default|GetSphere3))
  (bind _sphere (Variables|Default|GetSphere))
  (bind _sphere1 (Variables|Default|GetSphere1))
  (bind _sphere2 (Variables|Default|GetSphere2))
  (bind _sphere8 (Variables|Default|GetSphere8))
  (bind _sphere4 (Variables|Default|GetSphere4))
  (bind _sphere5 (Variables|Default|GetSphere5))
  (bind _sphere6 (Variables|Default|GetSphere6))
  (bind _sphere7 (Variables|Default|GetSphere7))
  (bind _array (Utilities|Array|MakeArray _sphere _sphere1 _sphere2 _sphere3 _sphere4 _sphere5 _sphere6 _sphere7 _sphere8))
  ;[0 0.1828 1] Start
  (bind _asmy_aic (Utilities|Casting|CastToMy_AIC (AI|GetAIController self)))
  (Default|SetupAIC _asmy_aic (Variables|Default|GetBT) (Game|Player|GetPlayerPawn 0) (Variables|Patroling|GetPartoler?))
  (bind _returnvalue (UserInterface|CreateWidget "/Game/PureBP/UI/BP/WP_FadeAuNoir.WP_FadeAuNoir_C"))
  (UserInterface|Viewport|AddtoViewport _returnvalue 0)
  (Variables|REF|SetREF_Fade _returnvalue)
  (Variables|REF|SetREF_Origin (Transformation|GetActorLocation))
  (bind _asbp_gi (CallFunction|RecupDispatcher))
  (EventDispatchers|UnbindallEventsfromResetAfterDie _asbp_gi)
  (bind _asbp_gi_2 (CallFunction|RecupDispatcher))
  (bind _output_get (Variables|Default|SetREF%20BP%20GI _asbp_gi_2))
  (EventDispatchers|BindEventtoPausewhenReadLore _output_get (delegate Custom|FixWhenReading))
  (EventDispatchers|BindEventtoUnPauseAfterRead (Variables|Default|GetREF%20BP%20GI) (delegate Custom|UnFixAfterRead))
  (EventDispatchers|BindEventtoCinematic (Variables|Default|GetREF%20BP%20GI) (delegate Custom|FixCinematic))
  (EventDispatchers|BindEventtoUnCinematic (Variables|Default|GetREF%20BP%20GI) (delegate Custom|UnFixCinematic))
  (Variables|Default|SetArrayDetectZone _array)
  (Variables|Default|SetNbZoneDetect (Utilities|Array|Length _array))
  (CallFunction|InteractSmoke false))

(event EventLighter
  ;[1 0.9448 0] Lighted
  (CallFunction|Lightedeuh))

(fn ConstructionScript
  (Utilities|Array|Clear (Variables|Patroling|GetPatrolPoints))
  (for _index (range 0 (Spline|GetNumberOfSplinePoints (Variables|Default|GetSpline)))
    (Utilities|Array|Add (Variables|Patroling|GetPatrolPoints) (Spline|GetLocationatSplinePoint (Variables|Default|GetSpline) _index "World"))))