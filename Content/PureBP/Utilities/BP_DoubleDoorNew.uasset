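; Interactive double door that the first-person player opens and closes, with an optional key lock.
; Front and back overlap volumes track range and player side, selecting which of two timelines swings both leaves in opposite yaw directions, with sound.
; Cursor events show a W_DoorInteract prompt based on door and lock state, which gates interaction.
; Interacting with a keyed door clears the player's key and HUD icon and releases the lock.
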(event OnComponentBeginOverlap(Front)
  (params (OverlappedComponent :type Primitive%20Component%20Object%20Reference) (OtherActor :type Actor%20Object%20Reference) (OtherComp :type Primitive%20Component%20Object%20Reference) (OtherBodyIndex :type Integer) (bFromSweep :type Boolean) (SweepResult :type Hit%20Result%20Structure%20%28by%20ref%29))
  ;[1 1 1] FRONT
  (Utilities|Casting|CastToBoxComponent OtherComp
    (:CastFailed
      (Utilities|Casting|CastToSphereComponent OtherComp
        (:CastFailed
          (bind _asfirst_person_character (Utilities|Casting|CastToFirstPersonCharacter OtherActor))
          (Variables|Default|SetREF%20First%20Person%20Character _asfirst_person_character)
          (Variables|Default|SetInRange true)
          (Variables|Default|SetPoseFromDoor "NewEnumerator0"))))))

(event OnComponentEndOverlap(Front)
  (params (OverlappedComponent :type Primitive%20Component%20Object%20Reference) (OtherActor :type Actor%20Object%20Reference) (OtherComp :type Primitive%20Component%20Object%20Reference) (OtherBodyIndex :type Integer))
  ;[1 1 1] FRONT
  (Utilities|Casting|CastToBoxComponent OtherComp
    (:CastFailed
      (Utilities|Casting|CastToSphereComponent OtherComp
        (:CastFailed
          (Utilities|Casting|CastToFirstPersonCharacter OtherActor)
          (Variables|Default|SetInRange false)
          (Variables|Default|SetPoseFromDoor "NewEnumerator3"))))))

(event OnComponentEndOverlap(Back)
  (params (OverlappedComponent :type Primitive%20Component%20Object%20Reference) (OtherActor :type Actor%20Object%20Reference) (OtherComp :type Primitive%20Component%20Object%20Reference) (OtherBodyIndex :type Integer))
  ;[1 1 1] BACK
  (Utilities|Casting|CastToBoxComponent OtherComp
    (:CastFailed
      (Utilities|Casting|CastToSphereComponent OtherComp
        (:CastFailed
          (Utilities|Casting|CastToFirstPersonCharacter OtherActor)
          (Variables|Default|SetInRange false)
          (Variables|Default|SetPoseFromDoor "NewEnumerator3"))))))

(event OnComponentBeginOverlap(Front1)
  (params (OverlappedComponent :type Primitive%20Component%20Object%20Reference) (OtherActor :type Actor%20Object%20Reference) (OtherComp :type Primitive%20Component%20Object%20Reference) (OtherBodyIndex :type Integer) (bFromSweep :type Boolean) (SweepResult :type Hit%20Result%20Structure%20%28by%20ref%29))
  ;[1 1 1] Comment
  (Utilities|Casting|CastToBoxComponent OtherComp
    (:CastFailed
      (Utilities|Casting|CastToSphereComponent OtherComp
        (:CastFailed
          (bind _asfirst_person_character (Utilities|Casting|CastToFirstPersonCharacter OtherActor))
          (Variables|Default|SetREF%20First%20Person%20Character _asfirst_person_character)
          (Variables|Default|SetInRange true)
          (Variables|Default|SetPoseFromDoor "NewEnumerator0"))))))

(event OnComponentBeginOverlap(Back)
  (params (OverlappedComponent :type Primitive%20Component%20Object%20Reference) (OtherActor :type Actor%20Object%20Reference) (OtherComp :type Primitive%20Component%20Object%20Reference) (OtherBodyIndex :type Integer) (bFromSweep :type Boolean) (SweepResult :type Hit%20Result%20Structure%20%28by%20ref%29))
  ;[1 1 1] BACK
  (Utilities|Casting|CastToBoxComponent OtherComp
    (:CastFailed
      (Utilities|Casting|CastToSphereComponent OtherComp
        (:CastFailed
          (bind _asfirst_person_character (Utilities|Casting|CastToFirstPersonCharacter OtherActor))
          (Variables|Default|SetREF%20First%20Person%20Character _asfirst_person_character)
          (Variables|Default|SetInRange true)
          (Variables|Default|SetPoseFromDoor "NewEnumerator1"))))))

(event OnComponentEndOverlap(Front1)
  (params (OverlappedComponent :type Primitive%20Component%20Object%20Reference) (OtherActor :type Actor%20Object%20Reference) (OtherComp :type Primitive%20Component%20Object%20Reference) (OtherBodyIndex :type Integer))
  ;[1 1 1] Comment
  (Utilities|Casting|CastToBoxComponent OtherComp
    (:CastFailed
      (Utilities|Casting|CastToSphereComponent OtherComp
        (:CastFailed
          (Utilities|Casting|CastToFirstPersonCharacter OtherActor)
          (Variables|Default|SetInRange false)
          (Variables|Default|SetPoseFromDoor "NewEnumerator3"))))))

(event OnComponentBeginOverlap(Back1)
  (params (OverlappedComponent :type Primitive%20Component%20Object%20Reference) (OtherActor :type Actor%20Object%20Reference) (OtherComp :type Primitive%20Component%20Object%20Reference) (OtherBodyIndex :type Integer) (bFromSweep :type Boolean) (SweepResult :type Hit%20Result%20Structure%20%28by%20ref%29))
  ;[1 1 1] Comment
  (Utilities|Casting|CastToBoxComponent OtherComp
    (:CastFailed
      (Utilities|Casting|CastToSphereComponent OtherComp
        (:CastFailed
          (bind _asfirst_person_character (Utilities|Casting|CastToFirstPersonCharacter OtherActor))
          (Variables|Default|SetREF%20First%20Person%20Character _asfirst_person_character)
          (Variables|Default|SetInRange true)
          (Variables|Default|SetPoseFromDoor "NewEnumerator1"))))))

(event OnComponentEndOverlap(Back1)
  (params (OverlappedComponent :type Primitive%20Component%20Object%20Reference) (OtherActor :type Actor%20Object%20Reference) (OtherComp :type Primitive%20Component%20Object%20Reference) (OtherBodyIndex :type Integer))
  ;[1 1 1] Comment
  (Utilities|Casting|CastToBoxComponent OtherComp
    (:CastFailed
      (Utilities|Casting|CastToSphereComponent OtherComp
        (:CastFailed
          (Utilities|Casting|CastToFirstPersonCharacter OtherActor)
          (Variables|Default|SetInRange false)
          (Variables|Default|SetPoseFromDoor "NewEnumerator3"))))))

(event Custom|InteractDoor
  (bind _returnvalue (Transformation|GetActorLocation))
  ;[1 1 1] Moving Door Interaction
  (if (not (Variables|Default|GetKey?))
    _
    (else
      (CallFunction|KillKey)))
  (if (Variables|Default|GetInRange)
    (switch Utilities|FlowControl|Switch|SwitchonEN_PosFromDoor (Variables|Default|GetPoseFromDoor)
      (:NewEnumerator0
        (switch Utilities|FlowControl|Switch|SwitchonEN_ModeOpenDoor (Variables|Default|GetDoorMode)
          (:NewEnumerator0
            (Audio|PlaySoundatLocation "/Game/SND/Bank/Door/SC_DoorOpen.SC_DoorOpen" _returnvalue "0, 0, 0" 1.0 1.0 0.0 0 0 0 0)
            (bind _openthedoor (Timeline|TimeOpenDoor Play)
              (:Update
                (Transformation|SetRelativeRotation (Variables|Default|GetR_Door) (Math|Rotator|MakeRotator 0.0 0.0 (Math|Float|Lerp 0.0 9e+01 _openthedoor)) false false)
                (Transformation|SetRelativeRotation (Variables|Default|GetL_Door) (Math|Rotator|MakeRotator 0.0 0.0 (Math|Float|Lerp 0.0 -9e+01 _openthedoor)) false false))
              (:Finished
                (switch Utilities|FlowControl|Switch|SwitchonEN_ModeOpenDoor (Variables|Default|GetDoorMode)
                  (:NewEnumerator0
                    (Variables|Default|SetDoorMode "NewEnumerator1"))
                  (:NewEnumerator1
                    (Variables|Default|SetDoorMode "NewEnumerator0"))))))
          (:NewEnumerator1
            (Audio|PlaySoundatLocation "/Game/SND/Bank/Door/SC_DoorClose.SC_DoorClose" _returnvalue "0, 0, 0" 1.0 1.0 0.0 0 0 0 0 :!label _label)
            (Timeline|TimeOpenDoor Reverse))
          (:NewEnumerator2
            (Audio|PlaySoundatLocation "/Game/SND/Bank/Door/SC_DoorClose.SC_DoorClose" _returnvalue "0, 0, 0" 1.0 1.0 0.0 0 0 0 0 :!label _label_2)
            (bind _openthedoor_2 (Timeline|Timeline_0 Reverse)
              (:Update
                (Transformation|SetRelativeRotation (Variables|Default|GetR_Door) (Math|Rotator|MakeRotator 0.0 0.0 (Math|Float|Lerp 0.0 -9e+01 _openthedoor_2)) false false)
                (Transformation|SetRelativeRotation (Variables|Default|GetL_Door) (Math|Rotator|MakeRotator 0.0 0.0 (Math|Float|Lerp 0.0 9e+01 _openthedoor_2)) false false))
              (:Finished
                (switch Utilities|FlowControl|Switch|SwitchonEN_ModeOpenDoor (Variables|Default|GetDoorMode)
                  (:NewEnumerator0
                    (Variables|Default|SetDoorMode "NewEnumerator2"))
                  (:NewEnumerator2
                    (Variables|Default|SetDoorMode "NewEnumerator0"))))))))
      (:NewEnumerator1
        (switch Utilities|FlowControl|Switch|SwitchonEN_ModeOpenDoor (Variables|Default|GetDoorMode)
          (:NewEnumerator0
            (Audio|PlaySoundatLocation "/Game/SND/Bank/Door/SC_DoorOpen.SC_DoorOpen" _returnvalue "0, 0, 0" 1.0 1.0 0.0 0 0 0 0)
            (Timeline|Timeline_0 Play))
          (:NewEnumerator1
            (goto _label))
          (:NewEnumerator2
            (goto _label_2)))))))

(event Custom|WichHud
  ;[1 1 1] WICH HUD
  (switch Utilities|FlowControl|Switch|SwitchonEN_ModeOpenDoor (Variables|Default|GetDoorMode)
    (:NewEnumerator0
      (CallFunction|HudOpenDoor))
    (:NewEnumerator1
      (CallFunction|HudCloseDoor :!label _label))
    (:NewEnumerator2
      (goto _label))))

(event Custom|HudOpenDoor
  ;[1 1 1] Choose HUD
  (if (not (Variables|Default|GetKey?))
    (Variables|Default|SetInteractable? true :!label _label)
    (Default|AppearDoorInteract (Variables|Default|GetREF_HudDoor) "[F] To Open Door" "Hidden" "Visible" "Hidden")
    (elif (not (Variables|Default|GetLock?))
      (goto _label)
      (elif (Variables|/Game/PureBP/Player/FirstPersonCharacter.FirstPersonCharacter_C|GetGotKey? (Variables|Default|GetREF%20First%20Person%20Character))
        (Variables|Default|SetInteractable? true)
        (Default|AppearDoorUnlocked (Variables|Default|GetREF_HudDoor) "Hidden" "Hidden" "[F] To Open Door")
        (else
          (Variables|Default|SetInteractable? false)
          (Default|AppearDoorInteract (Variables|Default|GetREF_HudDoor) "You need the KEY" "Visible" "Hidden" "Visible")))))
  (Variables|Default|SetAldyCreated? true))

(event Custom|HudCloseDoor
  ;[1 1 1] Choose HUD
  (Variables|Default|SetInteractable? true)
  (Default|AppearDoorInteract (Variables|Default|GetREF_HudDoor) "[F] To Close Door" "Hidden" "Visible" "Hidden"))

(event Custom|KillKey
  (bind _ref_first_person_character (Variables|Default|GetREF%20First%20Person%20Character))
  ;[1 1 1] Moving Door Interaction
  ;;[1 0.8745 0] Key Gest
  (Default|KilKey (Variables|/Game/PureBP/Player/FirstPersonCharacter.FirstPersonCharacter_C|GetREF_MainHud _ref_first_person_character))
  (Variables|/Game/PureBP/Player/FirstPersonCharacter.FirstPersonCharacter_C|SetGotKey? _ref_first_person_character false)
  (Variables|Default|SetLock? false))

(event EventUnCursored
  ;[1 1 1] Get Cursor
  (Default|DesappearDoorInteract (Variables|Default|GetREF_HudDoor))
  (Variables|Default|SetInteractable? false)
  (Variables|Default|SetAldyCreated? false))

(event EventCursored
  ;[1 1 1] Get Cursor
  (if (Variables|Default|GetInRange)
    (if (not (Variables|Default|GetAldyCreated?))
      (CallFunction|WichHud))))

(event EventBeginPlay
  ;[1 1 1] GET REF
  (bind _returnvalue (UserInterface|CreateWidget "/Game/PureBP/UI/BP/W_DoorInteract.W_DoorInteract_C"))
  (bind _output_get (Variables|Default|SetREF_HudDoor _returnvalue))
  (UserInterface|Viewport|AddtoViewport _output_get 0)
  (if (Variables|Default|GetKey?)
    (Variables|Default|SetLock? true)
    (else
      (Variables|Default|SetLock? false))))

(event EventInteract
  ;[1 1 1] Comment
  (if (Variables|Default|GetInteractable?)
    (CallFunction|InteractDoor)))

(fn ConstructionScript)