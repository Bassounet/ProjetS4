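; Interactive double door that the first-person player opens, closes or kicks in by running into it, with optional key lock.
; Front and back triggers record the player's side, picking one of two timelines that swing both leaves in opposite yaw directions.
; Interact and KickDoor check the key before driving them, kicks playing faster with camera shake.
; Cursor events update prompts and hand/padlock icons, and a dispatcher bound on front overlap reverses the door after death.
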(event OnComponentBeginOverlap(Front)
  (params (OverlappedComponent :type Primitive%20Component%20Object%20Reference) (OtherActor :type Actor%20Object%20Reference) (OtherComp :type Primitive%20Component%20Object%20Reference) (OtherBodyIndex :type Integer) (bFromSweep :type Boolean) (SweepResult :type Hit%20Result%20Structure%20%28by%20ref%29))
  ;[1 1 1] DETECT
  (Variables|Default|SetIsInRange? true)
  (Utilities|Casting|CastToSphereComponent OtherComp
    (:CastFailed
      (Utilities|Casting|CastToBoxComponent OtherComp
        (:CastFailed
          (bind _asfirst_person_character (Utilities|Casting|CastToFirstPersonCharacter OtherActor))
          (Variables|REF|SetREF_FP _asfirst_person_character)
          (Variables|Default|SetInRangeForOpen true)
          (Variables|Default|SetBack/Front "NewEnumerator0")
          (bind _asbp_gi (CallFunction|RecupDispatcher))
          (EventDispatchers|BindEventtoResetAfterDie _asbp_gi (delegate Custom|CloseDoor)))))))

(event OnComponentBeginOverlap(Back)
  (params (OverlappedComponent :type Primitive%20Component%20Object%20Reference) (OtherActor :type Actor%20Object%20Reference) (OtherComp :type Primitive%20Component%20Object%20Reference) (OtherBodyIndex :type Integer) (bFromSweep :type Boolean) (SweepResult :type Hit%20Result%20Structure%20%28by%20ref%29))
  ;[1 1 1] Interaction Porte Arrière
  (Variables|Default|SetIsInRange? true)
  (Utilities|Casting|CastToBoxComponent OtherComp
    (:CastFailed
      (Utilities|Casting|CastToFirstPersonCharacter OtherActor)
      (Variables|Default|SetInRangeForOpen true)
      (Variables|Default|SetBack/Front "NewEnumerator1"))))

(event OnComponentEndOverlap(Front)
  (params (OverlappedComponent :type Primitive%20Component%20Object%20Reference) (OtherActor :type Actor%20Object%20Reference) (OtherComp :type Primitive%20Component%20Object%20Reference) (OtherBodyIndex :type Integer))
  ;[1 1 1] DETECT
  (Variables|Default|SetIsInRange? false)
  (Utilities|Casting|CastToSphereComponent OtherComp
    (:CastFailed
      (Utilities|Casting|CastToBoxComponent OtherComp
        (:CastFailed
          (Utilities|Casting|CastToFirstPersonCharacter OtherActor)
          (Variables|Default|SetInRangeForOpen false)
          (CallFunction|HUDDoorOFF))))))

(event OnComponentEndOverlap(Back)
  (params (OverlappedComponent :type Primitive%20Component%20Object%20Reference) (OtherActor :type Actor%20Object%20Reference) (OtherComp :type Primitive%20Component%20Object%20Reference) (OtherBodyIndex :type Integer))
  ;[1 1 1] Interaction Porte Arrière
  (Variables|Default|SetIsInRange? false)
  (Utilities|Casting|CastToBoxComponent OtherComp
    (:CastFailed
      (Utilities|Casting|CastToFirstPersonCharacter OtherActor)
      (CallFunction|HUDDoorOFF)
      (Variables|Default|SetInRangeForOpen false))))

(event OnComponentBeginOverlap(Collision1)
  (params (OverlappedComponent :type Primitive%20Component%20Object%20Reference) (OtherActor :type Actor%20Object%20Reference) (OtherComp :type Primitive%20Component%20Object%20Reference) (OtherBodyIndex :type Integer) (bFromSweep :type Boolean) (SweepResult :type Hit%20Result%20Structure%20%28by%20ref%29))
  ;[1 1 1] DETECT
  (Utilities|Casting|CastToSphereComponent OtherComp
    (:CastFailed
      (Utilities|Casting|CastToBoxComponent OtherComp
        (:CastFailed
          (bind _asfirst_person_character (Utilities|Casting|CastToFirstPersonCharacter OtherActor))
          (Variables|Default|SetInRangeForOpen true)
          (if (Variables|/Game/PureBP/Player/FirstPersonCharacter.FirstPersonCharacter_C|GetIsRunning _asfirst_person_character)
            (switch Utilities|FlowControl|Switch|SwitchonEN_ModeOpenDoor (Variables|Default|GetModeOpened)
              (:NewEnumerator0
                (CallFunction|KickDoor)))))))))

(event OnComponentBeginOverlap(Collision2)
  (params (OverlappedComponent :type Primitive%20Component%20Object%20Reference) (OtherActor :type Actor%20Object%20Reference) (OtherComp :type Primitive%20Component%20Object%20Reference) (OtherBodyIndex :type Integer) (bFromSweep :type Boolean) (SweepResult :type Hit%20Result%20Structure%20%28by%20ref%29))
  ;[1 1 1] Interaction Porte Arrière
  (Utilities|Casting|CastToBoxComponent OtherComp
    (:CastFailed
      (bind _asfirst_person_character (Utilities|Casting|CastToFirstPersonCharacter OtherActor))
      (Variables|Default|SetInRangeForOpen true)
      (if (Variables|/Game/PureBP/Player/FirstPersonCharacter.FirstPersonCharacter_C|GetIsRunning _asfirst_person_character)
        (switch Utilities|FlowControl|Switch|SwitchonEN_ModeOpenDoor (Variables|Default|GetModeOpened)
          (:NewEnumerator0
            (CallFunction|KickDoor)))))))

(event Custom|KickDoor
  (bind _returnvalue (Transformation|GetActorLocation))
  ;[1 1 1] Open the door
  (if (Variables|Default|GetIsPlayingSound?)
    (if (not (Variables|Default|GetKey?))
      (Components|Timeline|SetPlayRate (Variables|Default|GetTimeToOpenDoor) 1e+01 :!label _label)
      (CallFunction|CamShakeLight)
      (switch Utilities|FlowControl|Switch|SwitchonEN_PosFromDoor (Variables|Default|GetBack/Front)
        (:NewEnumerator0
          (switch Utilities|FlowControl|Switch|SwitchonEN_ModeOpenDoor (Variables|Default|GetModeOpened)
            (:NewEnumerator0
              (bind _returnvalue_2 (Actor|GetActorOfClass "/Game/PureBP/Player/FirstPersonCharacter.FirstPersonCharacter_C"))
              (if (not (Variables|/Game/PureBP/Player/FirstPersonCharacter.FirstPersonCharacter_C|GetIsRunning _returnvalue_2))
                (Audio|PlaySoundatLocation "/Game/SND/Bank/Door/SC_DoorOpen.SC_DoorOpen" _returnvalue "0, 0, 0" 1.0 1.0 0.0 0 0 0 0)
                (else
                  (Audio|PlaySoundatLocation "/Game/StarterContent/Audio/Explosion01.Explosion01" _returnvalue "0, 0, 0" 1.0 1.0 0.0 0 0 0 0)))
              (Variables|Default|SetIsPlayingSound? false)
              (bind _openthedoor (Timeline|TimeToOpenDoor Play)
                (:Update
                  (Transformation|SetRelativeRotation (Variables|Default|GetStaticMesh) (Math|Rotator|MakeRotator 0.0 0.0 (Math|Float|Lerp 0.0 9e+01 _openthedoor)) false false)
                  (Transformation|SetRelativeRotation (Variables|Default|GetStaticMesh1) (Math|Rotator|MakeRotator 0.0 0.0 (Math|Float|Lerp 0.0 -9e+01 _openthedoor)) false false)
                  (if (Variables|Default|GetKey?) :!label _label_2
                    (bind _ref_mainhud (CallFunction|GetHUD))
                    (Widget|SetVisibility (Variables|/Game/PureBP/UI/BP/W_MainHud.W_MainHud_C|GetKey _ref_mainhud) "Hidden")
                    (bind _asfirst_person_character (CallFunction|GetPlayer))
                    (Variables|/Game/PureBP/Player/FirstPersonCharacter.FirstPersonCharacter_C|SetGotKey? _asfirst_person_character false)
                    (Variables|Default|SetLock? false)))
                (:Finished
                  (Variables|Default|SetIsPlayingSound? true)
                  (switch Utilities|FlowControl|Switch|SwitchonEN_ModeOpenDoor (Variables|Default|GetModeOpened)
                    (:NewEnumerator0
                      (Variables|Default|SetModeOpened "NewEnumerator1"))
                    (:NewEnumerator1
                      (Variables|Default|SetModeOpened "NewEnumerator0"))))))
            (:NewEnumerator1
              (Audio|PlaySoundatLocation "/Game/SND/Bank/Door/SC_DoorClose.SC_DoorClose" _returnvalue "0, 0, 0" 1.0 1.0 0.0 0 0 0 0 :!label _label_3)
              (Variables|Default|SetIsPlayingSound? false)
              (Timeline|TimeToOpenDoor Reverse))
            (:NewEnumerator2
              (Audio|PlaySoundatLocation "/Game/SND/Bank/Door/SC_DoorClose.SC_DoorClose" _returnvalue "0, 0, 0" 1.0 1.0 0.0 0 0 0 0 :!label _label_4)
              (Variables|Default|SetIsPlayingSound? false)
              (bind _openthedoor_2 (Timeline|Timeline_1 Reverse)
                (:Update
                  (Transformation|SetRelativeRotation (Variables|Default|GetStaticMesh) (Math|Rotator|MakeRotator 0.0 0.0 (Math|Float|Lerp 0.0 -9e+01 _openthedoor_2)) false false)
                  (Transformation|SetRelativeRotation (Variables|Default|GetStaticMesh1) (Math|Rotator|MakeRotator 0.0 0.0 (Math|Float|Lerp 0.0 9e+01 _openthedoor_2)) false false)
                  (goto _label_2))
                (:Finished
                  (Variables|Default|SetIsPlayingSound? true)
                  (switch Utilities|FlowControl|Switch|SwitchonEN_ModeOpenDoor (Variables|Default|GetModeOpened)
                    (:NewEnumerator0
                      (Variables|Default|SetModeOpened "NewEnumerator2"))
                    (:NewEnumerator2
                      (Variables|Default|SetModeOpened "NewEnumerator0"))))))))
        (:NewEnumerator1
          (switch Utilities|FlowControl|Switch|SwitchonEN_ModeOpenDoor (Variables|Default|GetModeOpened)
            (:NewEnumerator0
              (bind _returnvalue_3 (Actor|GetActorOfClass "/Game/PureBP/Player/FirstPersonCharacter.FirstPersonCharacter_C"))
              (if (not (Variables|/Game/PureBP/Player/FirstPersonCharacter.FirstPersonCharacter_C|GetIsRunning _returnvalue_3))
                (Audio|PlaySoundatLocation "/Game/SND/Bank/Door/SC_DoorOpen.SC_DoorOpen" _returnvalue "0, 0, 0" 1.0 1.0 0.0 0 0 0 0)
                (else
                  (Audio|PlaySoundatLocation "/Game/StarterContent/Audio/Explosion01.Explosion01" _returnvalue "0, 0, 0" 1.0 1.0 0.0 0 0 0 0)))
              (Variables|Default|SetIsPlayingSound? false)
              (Timeline|Timeline_1 Play))
            (:NewEnumerator1
              (goto _label_3))
            (:NewEnumerator2
              (goto _label_4)))))
      (else
        (bind _asfirst_person_character_2 (CallFunction|GetPlayer))
        (if (Variables|/Game/PureBP/Player/FirstPersonCharacter.FirstPersonCharacter_C|GetGotKey? _asfirst_person_character_2)
          (goto _label)
          (elif (not (Variables|Default|GetLock?))
            (goto _label)
            (else
              (Audio|PlaySoundatLocation "/Game/SND/Bank/Door/SC_DoorImpact.SC_DoorImpact" (Transformation|GetActorLocation) "0, 0, 0" 1.0 1.0 0.0 0 0 0 0)
              (CallFunction|CamShakeLight))))))))

(event Custom|AppearCadenaCursor
  (bind _ref_main_hud (Variables|Default|GetREF%20Main%20Hud))
  ;[1 1 1] Cursor Interaction
  (Widget|SetVisibility (Variables|/Game/PureBP/UI/BP/W_MainHud.W_MainHud_C|GetCadena _ref_main_hud) "Visible")
  (Widget|SetVisibility (Variables|/Game/PureBP/UI/BP/W_MainHud.W_MainHud_C|GetPrincipalCursor _ref_main_hud) "Hidden"))

(event Custom|HUDDoorOFF
  ;[1 1 1] HUD Gest
  (Widget|SetVisibility (Variables|REF|GetREF_WidgetDoorOpen) "Hidden"))

(event Custom|DoorState
  ;[1 1 1] Select Door State HUD
  (switch Utilities|FlowControl|Switch|SwitchonEN_DoorState (Variables|Default|GetSelectionDoorState)
    (:NewEnumerator0
      (CallFunction|AppearHandCursor :!label _label))
    (:NewEnumerator1
      (CallFunction|AppearCadenaCursor))
    (:NewEnumerator2
      (goto _label))))

(event Custom|ResetAfterDie
  ;[1 1 1] Open the door
  (Utilities|FlowControl|Sequence
    (:then_0
      (bind _openthedoor (Timeline|Timeline_1 Reverse)
        (:Update
          (Transformation|SetRelativeRotation (Variables|Default|GetStaticMesh) (Math|Rotator|MakeRotator 0.0 0.0 (Math|Float|Lerp 0.0 -9e+01 _openthedoor)) false false)
          (Transformation|SetRelativeRotation (Variables|Default|GetStaticMesh1) (Math|Rotator|MakeRotator 0.0 0.0 (Math|Float|Lerp 0.0 9e+01 _openthedoor)) false false)
          (if (Variables|Default|GetKey?) :!label _label
            (bind _ref_mainhud (CallFunction|GetHUD))
            (Widget|SetVisibility (Variables|/Game/PureBP/UI/BP/W_MainHud.W_MainHud_C|GetKey _ref_mainhud) "Hidden")
            (bind _asfirst_person_character (CallFunction|GetPlayer))
            (Variables|/Game/PureBP/Player/FirstPersonCharacter.FirstPersonCharacter_C|SetGotKey? _asfirst_person_character false)
            (Variables|Default|SetLock? false)))
        (:Finished
          (Variables|Default|SetIsPlayingSound? true)
          (switch Utilities|FlowControl|Switch|SwitchonEN_ModeOpenDoor (Variables|Default|GetModeOpened)
            (:NewEnumerator0
              (Variables|Default|SetModeOpened "NewEnumerator2"))
            (:NewEnumerator2
              (Variables|Default|SetModeOpened "NewEnumerator0"))))))
    (:then_1
      (bind _openthedoor_2 (Timeline|TimeToOpenDoor Reverse)
        (:Update
          (Transformation|SetRelativeRotation (Variables|Default|GetStaticMesh) (Math|Rotator|MakeRotator 0.0 0.0 (Math|Float|Lerp 0.0 9e+01 _openthedoor_2)) false false)
          (Transformation|SetRelativeRotation (Variables|Default|GetStaticMesh1) (Math|Rotator|MakeRotator 0.0 0.0 (Math|Float|Lerp 0.0 -9e+01 _openthedoor_2)) false false)
          (goto _label))
        (:Finished
          (Variables|Default|SetIsPlayingSound? true)
          (switch Utilities|FlowControl|Switch|SwitchonEN_ModeOpenDoor (Variables|Default|GetModeOpened)
            (:NewEnumerator0
              (Variables|Default|SetModeOpened "NewEnumerator1"))
            (:NewEnumerator1
              (Variables|Default|SetModeOpened "NewEnumerator0"))))))))

(event Custom|DoorActivate
  (bind _returnvalue (Transformation|GetActorLocation))
  ;[1 1 1] Open the door
  (if (Variables|Default|GetIsPlayingSound?)
    (Components|Timeline|SetPlayRate (Variables|Default|GetTimeToOpenDoor) 1.0)
    (if (Variables|Default|GetInRangeForOpen)
      (switch Utilities|FlowControl|Switch|SwitchonEN_PosFromDoor (Variables|Default|GetBack/Front)
        (:NewEnumerator0
          (switch Utilities|FlowControl|Switch|SwitchonEN_ModeOpenDoor (Variables|Default|GetModeOpened)
            (:NewEnumerator0
              (bind _returnvalue_2 (Actor|GetActorOfClass "/Game/PureBP/Player/FirstPersonCharacter.FirstPersonCharacter_C"))
              (if (not (Variables|/Game/PureBP/Player/FirstPersonCharacter.FirstPersonCharacter_C|GetIsRunning _returnvalue_2))
                (Audio|PlaySoundatLocation "/Game/SND/Bank/Door/SC_DoorOpen.SC_DoorOpen" _returnvalue "0, 0, 0" 1.0 1.0 0.0 0 0 0 0)
                (else
                  (Audio|PlaySoundatLocation "/Game/StarterContent/Audio/Explosion01.Explosion01" _returnvalue "0, 0, 0" 1.0 1.0 0.0 0 0 0 0)))
              (Variables|Default|SetIsPlayingSound? false)
              (bind _openthedoor (Timeline|TimeToOpenDoor Play)
                (:Update
                  (Transformation|SetRelativeRotation (Variables|Default|GetStaticMesh) (Math|Rotator|MakeRotator 0.0 0.0 (Math|Float|Lerp 0.0 9e+01 _openthedoor)) false false)
                  (Transformation|SetRelativeRotation (Variables|Default|GetStaticMesh1) (Math|Rotator|MakeRotator 0.0 0.0 (Math|Float|Lerp 0.0 -9e+01 _openthedoor)) false false)
                  (if (Variables|Default|GetKey?) :!label _label
                    (bind _ref_mainhud (CallFunction|GetHUD))
                    (Widget|SetVisibility (Variables|/Game/PureBP/UI/BP/W_MainHud.W_MainHud_C|GetKey _ref_mainhud) "Hidden")
                    (bind _asfirst_person_character (CallFunction|GetPlayer))
                    (Variables|/Game/PureBP/Player/FirstPersonCharacter.FirstPersonCharacter_C|SetGotKey? _asfirst_person_character false)
                    (Variables|Default|SetLock? false)))
                (:Finished
                  (Variables|Default|SetIsPlayingSound? true)
                  (switch Utilities|FlowControl|Switch|SwitchonEN_ModeOpenDoor (Variables|Default|GetModeOpened)
                    (:NewEnumerator0
                      (Variables|Default|SetModeOpened "NewEnumerator1"))
                    (:NewEnumerator1
                      (Variables|Default|SetModeOpened "NewEnumerator0"))))))
            (:NewEnumerator1
              (Audio|PlaySoundatLocation "/Game/SND/Bank/Door/SC_DoorClose.SC_DoorClose" _returnvalue "0, 0, 0" 1.0 1.0 0.0 0 0 0 0 :!label _label_2)
              (Variables|Default|SetIsPlayingSound? false)
              (Timeline|TimeToOpenDoor Reverse))
            (:NewEnumerator2
              (Audio|PlaySoundatLocation "/Game/SND/Bank/Door/SC_DoorClose.SC_DoorClose" _returnvalue "0, 0, 0" 1.0 1.0 0.0 0 0 0 0 :!label _label_3)
              (Variables|Default|SetIsPlayingSound? false)
              (bind _openthedoor_2 (Timeline|Timeline_1 Reverse)
                (:Update
                  (Transformation|SetRelativeRotation (Variables|Default|GetStaticMesh) (Math|Rotator|MakeRotator 0.0 0.0 (Math|Float|Lerp 0.0 -9e+01 _openthedoor_2)) false false)
                  (Transformation|SetRelativeRotation (Variables|Default|GetStaticMesh1) (Math|Rotator|MakeRotator 0.0 0.0 (Math|Float|Lerp 0.0 9e+01 _openthedoor_2)) false false)
                  (goto _label))
                (:Finished
                  (Variables|Default|SetIsPlayingSound? true)
                  (switch Utilities|FlowControl|Switch|SwitchonEN_ModeOpenDoor (Variables|Default|GetModeOpened)
                    (:NewEnumerator0
                      (Variables|Default|SetModeOpened "NewEnumerator2"))
                    (:NewEnumerator2
                      (Variables|Default|SetModeOpened "NewEnumerator0"))))))))
        (:NewEnumerator1
          (switch Utilities|FlowControl|Switch|SwitchonEN_ModeOpenDoor (Variables|Default|GetModeOpened)
            (:NewEnumerator0
              (bind _returnvalue_3 (Actor|GetActorOfClass "/Game/PureBP/Player/FirstPersonCharacter.FirstPersonCharacter_C"))
              (if (not (Variables|/Game/PureBP/Player/FirstPersonCharacter.FirstPersonCharacter_C|GetIsRunning _returnvalue_3))
                (Audio|PlaySoundatLocation "/Game/SND/Bank/Door/SC_DoorOpen.SC_DoorOpen" _returnvalue "0, 0, 0" 1.0 1.0 0.0 0 0 0 0)
                (else
                  (Audio|PlaySoundatLocation "/Game/StarterContent/Audio/Explosion01.Explosion01" _returnvalue "0, 0, 0" 1.0 1.0 0.0 0 0 0 0)))
              (Variables|Default|SetIsPlayingSound? false)
              (Timeline|Timeline_1 Play))
            (:NewEnumerator1
              (goto _label_2))
            (:NewEnumerator2
              (goto _label_3))))))))

(event Custom|DisappearCursor
  (bind _ref_main_hud (Variables|Default|GetREF%20Main%20Hud))
  ;[1 1 1] Cursor Interaction
  (Widget|SetVisibility (Variables|/Game/PureBP/UI/BP/W_MainHud.W_MainHud_C|GetCadena _ref_main_hud) "Hidden")
  (Widget|SetVisibility (Variables|/Game/PureBP/UI/BP/W_MainHud.W_MainHud_C|GetPrincipalCursor _ref_main_hud) "Visible"))

(event Custom|AppearHandCursor
  (bind _ref_main_hud (Variables|Default|GetREF%20Main%20Hud))
  ;[1 1 1] Cursor Interaction
  (if (Variables|Default|GetIsInRange?)
    (Widget|SetVisibility (Variables|/Game/PureBP/UI/BP/W_MainHud.W_MainHud_C|GetCadena _ref_main_hud) "Hidden")
    (Widget|SetVisibility (Variables|/Game/PureBP/UI/BP/W_MainHud.W_MainHud_C|GetHand _ref_main_hud) "Visible")))

(event Custom|HUD_OpenDoor
  (bind _ref_widgetdooropen (Variables|REF|GetREF_WidgetDoorOpen))
  (bind _ref_widgetdooropen_2 (Variables|REF|GetREF_WidgetDoorOpen))
  ;[1 1 1] HUD Gest
  (if (Variables|Default|GetIsInRange?)
    (if (not (Variables|Default|GetKey?))
      (Widget|SetVisibility _ref_widgetdooropen_2 "Visible" :!label _label)
      (Rendering|Components|TextRender|SetText (Variables|/Game/PureBP/UI/BP/W_DoorInteract.W_DoorInteract_C|GetTextBlock_0 _ref_widgetdooropen_2) "[F] To open door")
      (else
        (bind _asfirst_person_character (CallFunction|GetPlayer))
        (if (Variables|/Game/PureBP/Player/FirstPersonCharacter.FirstPersonCharacter_C|GetGotKey? _asfirst_person_character)
          (goto _label)
          (elif (not (Variables|Default|GetLock?))
            (goto _label)
            (else
              (Widget|SetVisibility _ref_widgetdooropen "Visible")
              (Rendering|Components|TextRender|SetText (Variables|/Game/PureBP/UI/BP/W_DoorInteract.W_DoorInteract_C|GetTextBlock_0 _ref_widgetdooropen) "Vous avez besoin de la clef"))))))))

(event Custom|HUDCloseDoor
  (bind _ref_widgetdooropen (Variables|REF|GetREF_WidgetDoorOpen))
  ;[1 1 1] HUD Gest
  (if (Variables|Default|GetIsInRange?)
    (Widget|SetVisibility _ref_widgetdooropen "Visible")
    (Rendering|Components|TextRender|SetText (Variables|/Game/PureBP/UI/BP/W_DoorInteract.W_DoorInteract_C|GetTextBlock_0 _ref_widgetdooropen) "[F] To close door")))

(event Custom|CloseDoor
  ;[1 1 1] DETECT
  (CallFunction|ResetAfterDie))

(event Custom|WichHUD
  ;[1 1 1] Select HUD
  (switch Utilities|FlowControl|Switch|SwitchonEN_ModeOpenDoor (Variables|Default|GetModeOpened)
    (:NewEnumerator0
      (CallFunction|HUDOpenDoor))
    (:NewEnumerator1
      (CallFunction|HUDCloseDoor))
    (:NewEnumerator2
      (CallFunction|HUDCloseDoor))))

(event EventBeginPlay
  ;[1 1 1] GetSomeRef
  (bind _returnvalue (UserInterface|CreateWidget "/Game/PureBP/UI/BP/W_DoorInteract.W_DoorInteract_C"))
  (Variables|REF|SetREF_WidgetDoorOpen _returnvalue)
  (UserInterface|Viewport|AddtoViewport (Variables|REF|GetREF_WidgetDoorOpen) 0)
  (Widget|SetVisibility (Variables|REF|GetREF_WidgetDoorOpen) "Hidden"))

(event EventInteract
  ;[1 1 1] Interaction
  (if (Variables|Default|GetIsInRange?)
    (if (not (Variables|Default|GetKey?))
      (CallFunction|DoorActivate :!label _label)
      (elif (not (Variables|Default|GetLock?))
        (goto _label)
        (else
          (bind _asfirst_person_character (CallFunction|GetPlayer))
          (if (Variables|/Game/PureBP/Player/FirstPersonCharacter.FirstPersonCharacter_C|GetGotKey? _asfirst_person_character)
            (goto _label)
            (else
              (Audio|PlaySound2D "/Game/SND/Bank/Door/Household_Door_Lock_Deadbolt_01.Household_Door_Lock_Deadbolt_01" 1.0 1.0 0.0 0 0))))))))

(event EventCursored
  ;[1 1 1] Cursor Interaction
  (if (Variables|Default|GetIsInRange?)
    (bind _ref_mainhud (CallFunction|GetHUD))
    (Variables|Default|SetREF%20Main%20Hud _ref_mainhud)
    (CallFunction|WichHUD)
    (if (Variables|Default|GetKey?)
      (if (not (Variables|Default|GetLock?))
        (Variables|Default|SetSelectionDoorState "NewEnumerator0" :!label _label)
        (else
          (bind _asfirst_person_character (CallFunction|GetPlayer))
          (if (Variables|/Game/PureBP/Player/FirstPersonCharacter.FirstPersonCharacter_C|GetGotKey? _asfirst_person_character)
            (Variables|Default|SetSelectionDoorState "NewEnumerator2")
            (else
              (Variables|Default|SetSelectionDoorState "NewEnumerator1")))))
      (else
        (goto _label)))
    (CallFunction|DoorState)
    (else
      (CallFunction|DisappearCursor))))

(event EventUnCursored
  ;[1 1 1] Cursor Interaction
  (CallFunction|HUDDoorOFF)
  (CallFunction|DisappearCursor))

(fn ConstructionScript)