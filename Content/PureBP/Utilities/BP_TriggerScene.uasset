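; BP_TriggerScene is a trigger volume that plays a one-time level sequence when the first-person character walks into its box.
; On overlap, Scene1 creates a player for the configured sequence, disables player input and starts playback.
; A timer set to the sequence's duration re-enables input afterwards, and the AldyPlayed flag stops the scene from replaying.
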(event OnComponentBeginOverlap(Box)
  (params (OverlappedComponent :type Primitive%20Component%20Object%20Reference) (OtherActor :type Actor%20Object%20Reference) (OtherComp :type Primitive%20Component%20Object%20Reference) (OtherBodyIndex :type Integer) (bFromSweep :type Boolean) (SweepResult :type Hit%20Result%20Structure%20%28by%20ref%29))
  (Utilities|Casting|CastToFirstPersonCharacter OtherActor)
  (CallFunction|Scene1))

(event Custom|CustomEvent
  (Input|EnableInput (Game|GetPlayerCharacter 0) (Game|GetPlayerController 0)))

(event Custom|Scene%201
  (if (not (Variables|Default|GetAldyPlayed?))
    (Utilities|FlowControl|Sequence
      (:then_0
        (bind _returnvalue (Sequencer|Player|CreateLevelSequencePlayer (Variables|Default|GetSequence%20à%20jouer)))
        (Variables|Default|SetRef_Sequence _returnvalue))
      (:then_1
        (Input|DisableInput (Game|GetPlayerCharacter 0) (Game|GetPlayerController 0))
        (Sequencer|Player|Play (Variables|Default|GetRef_Sequence) :!class /Script/MovieScene.MovieSceneSequencePlayer)
        (Utilities|Time|SetTimerbyEvent (delegate Custom|CustomEvent) (Class|TimeManagementBlueprintLibrary|ToSeconds(QualifiedFrameTime) (Media|MediaPlayer|GetDuration (Variables|Default|GetRef_Sequence))))
        (Variables|Default|SetAldyPlayed? true)))))

(fn ConstructionScript)