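; Inspectable lore object that the player picks up to examine and rotate in front of the first-person character.
; Cursor hover events swap the HUD crosshair for inspect prompts.
; Grip snaps it to the player's inspection zone, disables physics, hands input to the object for rotation, and calls a pause-for-reading dispatcher.
; UnGrip detaches the mesh, restores physics and player input, and unpauses; BeginPlay adds a lore widget to the viewport.
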(event Custom|UnGrip
  (bind _returnvalue (Game|GetPlayerController 0))
  (bind _staticmesh (Variables|Default|GetStaticMesh))
  ;[0 0.01975 1] UnGrip
  (Transformation|DetachFromComponent (Variables|Default|GetStaticMesh) "KeepWorld" "KeepWorld" "KeepWorld" true)
  (Variables|Default|SetGripped? false)
  (bind _asbp_gi (CallFunction|RecupDispatcher))
  (Default|CallUnPauseAfterRead _asbp_gi)
  (Collision|SetCollisionEnabled _staticmesh "QueryAndPhysics")
  (Physics|SetSimulatePhysics _staticmesh true)
  (Input|DisableInput _returnvalue)
  (Input|EnableInput (Variables|Default|GetREF%20First%20Person%20Character) _returnvalue))

(event Custom|Grip
  (bind _returnvalue (Game|GetPlayerController 0))
  (bind _staticmesh (Variables|Default|GetStaticMesh))
  ;[0 1 0.02873] GRIP
  (bind _asfirst_person_character (CallFunction|GetPlayer))
  (Variables|Default|SetREF%20First%20Person%20Character _asfirst_person_character)
  (Variables|Default|SetGripped? true)
  (bind _asbp_gi (CallFunction|RecupDispatcher))
  (Default|CallPausewhenReadLore _asbp_gi)
  (Transformation|AttachComponentToComponent (Variables|Default|GetDefaultSceneRoot) (Variables|/Game/PureBP/Player/FirstPersonCharacter.FirstPersonCharacter_C|GetZoneTeleportInspection (Variables|Default|GetREF%20First%20Person%20Character)) "None" "SnapToTarget" "SnapToTarget" "KeepRelative" true)
  (Physics|SetSimulatePhysics _staticmesh false)
  (Collision|SetCollisionEnabled _staticmesh "NoCollision")
  (Input|DisableInput (Variables|Default|GetREF%20First%20Person%20Character) _returnvalue)
  (Input|EnableInput _returnvalue))

(event EventBeginPlay
  ;[1 1 1] Comment
  (bind _returnvalue (UserInterface|CreateWidget "/Game/PureBP/UI/WP_LoreObject.WP_LoreObject_C"))
  (bind _output_get (Variables|Default|SetREF%20LoreHUD _returnvalue))
  (UserInterface|Viewport|AddtoViewport _output_get 0))

(event EventUnCursored
  (bind _ref_main_hud (Variables|Default|GetREF%20Main%20Hud))
  ;[1 1 1] Cursor Event
  (Widget|SetVisibility (Variables|/Game/PureBP/UI/W_MainHud.W_MainHud_C|GetInspect _ref_main_hud) "Hidden")
  (Widget|SetVisibility (Variables|/Game/PureBP/UI/W_MainHud.W_MainHud_C|GetPrincipalCursor _ref_main_hud) "Visible")
  (Variables|Default|SetLookAtMe? false))

(event EventCursored
  ;[1 1 1] Cursor Event
  (bind _ref_mainhud (CallFunction|GetHUD))
  (bind _output_get (Variables|Default|SetREF%20Main%20Hud _ref_mainhud))
  (Widget|SetVisibility (Variables|/Game/PureBP/UI/W_MainHud.W_MainHud_C|GetInspect _output_get) "Visible")
  (Widget|SetVisibility (Variables|/Game/PureBP/UI/W_MainHud.W_MainHud_C|GetPrincipalCursor _output_get) "Hidden")
  (Variables|Default|SetLookAtMe? true))

(event EventInteract
  ;[1 1 1] Gripping
  (if (not (Variables|Default|GetGripped?))
    (CallFunction|Grip)
    (else
      (CallFunction|UnGrip))))

(event Input|ActionEvents|InputActionInteract
  (params (Key :type Key%20Structure :default "None"))
  (:Pressed
    (if (Variables|Default|GetGripped?)
      (CallFunction|UnGrip))))

(event Input|AxisEvents|InputAxisTurn
  (params (AxisValue :type Float%20%28single-precision%29))
  ;[1 1 1] Rotate Item
  (Transformation|SetActorRotation (Math|Rotator|CombineRotators (Transformation|GetActorRotation) (Math|Rotator|MakeRotator 0.0 0.0 (* AxisValue -5.0)))))

(event Input|AxisEvents|InputAxisLookUp
  (params (AxisValue :type Float%20%28single-precision%29))
  ;[1 1 1] Rotate Item
  (Transformation|SetActorRotation (Math|Rotator|CombineRotators (Transformation|GetActorRotation) (Math|Rotator|MakeRotator 0.0 (* AxisValue -5.0) 0.0))))

(fn ConstructionScript)