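; Spring-loaded actor, apparently a poster, that snaps out when the first-person character enters its box and folds back when lit.
; Overlap calls Spoink, which plays a fast timeline that yaws the root toward NemAngle, then sets Open after a delay.
; Once Open, the Lighted event reverses the timeline more slowly, guarded by Replié.
; Open is never cleared here, so later overlaps do not spring it again.
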(event OnComponentBeginOverlap(Box)
  (params (OverlappedComponent :type Primitive%20Component%20Object%20Reference) (OtherActor :type Actor%20Object%20Reference) (OtherComp :type Primitive%20Component%20Object%20Reference) (OtherBodyIndex :type Integer) (bFromSweep :type Boolean) (SweepResult :type Hit%20Result%20Structure%20%28by%20ref%29))
  (Utilities|Casting|CastToFirstPersonCharacter OtherActor)
  (Development|PrintString "Spoink")
  (CallFunction|Spoink))

(event Custom|Spoink
  ;[1 1 1] Open/ Close
  (if (not (Variables|Default|GetOpen?))
    (Components|Timeline|SetPlayRate (Variables|Default|GetTimeline_0) 1e+01)
    (Variables|Default|SetReplié false)
    (bind _openthedoor (Timeline|Timeline_0 Play)
      (:Update
        (Transformation|SetRelativeRotation (Variables|Default|GetDefaultSceneRoot) (Math|Rotator|MakeRotator 0.0 0.0 (Math|Float|Lerp 0.0 (Variables|Default|GetNemAngle) _openthedoor)) false false))
      (:Finished
        (Utilities|FlowControl|Delay 3.0)
        (Variables|Default|SetOpen? true)))))

(event Custom|Lighted
  ;[1 1 1] Open/ Close
  (if (not (Variables|Default|GetReplié))
    (if (Variables|Default|GetOpen?)
      (Variables|Default|SetReplié true)
      (Components|Timeline|SetPlayRate (Variables|Default|GetTimeline_0) 2.0)
      (bind _openthedoor (Timeline|Timeline_0 Reverse)
        (:Update
          (Transformation|SetRelativeRotation (Variables|Default|GetDefaultSceneRoot) (Math|Rotator|MakeRotator 0.0 0.0 (Math|Float|Lerp 0.0 (Variables|Default|GetNemAngle) _openthedoor)) false false))
        (:Finished
          (Utilities|FlowControl|Delay 3.0)
          (Variables|Default|SetOpen? true))))))

(event EventBeginPlay)

(event Collision|EventActorBeginOverlap
  (params (OtherActor :type Actor%20Object%20Reference)))

(event EventTick
  (params (DeltaSeconds :type Float%20%28single-precision%29)))

(fn ConstructionScript)