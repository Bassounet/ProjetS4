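; BP_InteractDictaTest is an interactable actor that switches on the player's "Dicta" state and shows a configurable player line as a subtitle.
; Cursored and UnCursored swap the HUD's inspect and main cursors and set the look flag that gates Interact.
; A timer calls Reset to switch Dicta off and hide the subtitle, then a one-second delay clears the already-triggered flag to allow another interaction.
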(event Custom|Reset
  ;[1 1 1] What You said?
  (Default|DictaOFF (Variables|Default|GetREF_First%20Person%20Character))
  (Widget|SetVisibility (Variables|/Game/PureBP/UI/W_MainHud.W_MainHud_C|GetSous-Titres (Variables|Default|GetREF%20Main%20Hud)) "Hidden")
  (Utilities|FlowControl|RetriggerableDelay 1.0)
  (Variables|Default|SetAldyLook? false))

(event EventBeginPlay)

(event Collision|EventActorBeginOverlap
  (params (OtherActor :type Actor%20Object%20Reference)))

(event EventTick
  (params (DeltaSeconds :type Float%20%28single-precision%29)))

(event EventInteract
  ;[1 1 1] What You said?
  (if (Variables|Default|GetLookAtMe?)
    (if (not (Variables|Default|GetAldyLook?))
      (bind _returnvalue (Utilities|Time|SetTimerbyEvent (delegate Custom|Reset) (Variables|Default|GetTime%20To%20Wait%20before%20Text%20Desappear)))
      (Variables|Default|SetRefTimer _returnvalue)
      (bind _asfirst_person_character (CallFunction|GetPlayer))
      (bind _output_get (Variables|Default|SetREF_First%20Person%20Character _asfirst_person_character))
      (Default|DictaON _output_get)
      (Widget|SetVisibility (Variables|/Game/PureBP/UI/W_MainHud.W_MainHud_C|GetSous-Titres (Variables|Default|GetREF%20Main%20Hud)) "Visible")
      (Rendering|Components|TextRender|SetText (Variables|/Game/PureBP/UI/W_MainHud.W_MainHud_C|GetSous-Titres (Variables|Default|GetREF%20Main%20Hud)) (Variables|Default|GetText%20Player%20Say))
      (Variables|Default|SetAldyLook? true))))

(event EventCursored
  ;[1 1 1] Interaction
  (bind _ref_mainhud (CallFunction|GetHUD))
  (bind _output_get (Variables|Default|SetREF%20Main%20Hud _ref_mainhud))
  (Widget|SetVisibility (Variables|/Game/PureBP/UI/W_MainHud.W_MainHud_C|GetInspect _output_get) "Visible")
  (Widget|SetVisibility (Variables|/Game/PureBP/UI/W_MainHud.W_MainHud_C|GetPrincipalCursor _output_get) "Hidden")
  (Variables|Default|SetLookAtMe? true))

(event EventUnCursored
  (bind _ref_main_hud (Variables|Default|GetREF%20Main%20Hud))
  ;[1 1 1] Interaction
  (Widget|SetVisibility (Variables|/Game/PureBP/UI/W_MainHud.W_MainHud_C|GetInspect _ref_main_hud) "Hidden")
  (Widget|SetVisibility (Variables|/Game/PureBP/UI/W_MainHud.W_MainHud_C|GetPrincipalCursor _ref_main_hud) "Visible")
  (Variables|Default|SetLookAtMe? false))

(fn ConstructionScript)