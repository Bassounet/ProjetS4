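; BP_BatteryChoice is a battery pickup that adds a configurable charge to the first-person character.
; When the FirstPersonCharacter overlaps its Sphere, it creates a collectable UI widget and shows a French message with the percentage received.
; It then passes the BatteryToAdd amount and the widget reference to the character's GetBattery, and destroys itself.
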(event OnComponentBeginOverlap(Sphere)
  (params (OverlappedComponent :type Primitive%20Component%20Object%20Reference) (OtherActor :type Actor%20Object%20Reference) (OtherComp :type Primitive%20Component%20Object%20Reference) (OtherBodyIndex :type Integer) (bFromSweep :type Boolean) (SweepResult :type Hit%20Result%20Structure%20%28by%20ref%29))
  ;[1 1 1] Comment
  (bind _asfirst_person_character (Utilities|Casting|CastToFirstPersonCharacter OtherActor))
  (bind _returnvalue (UserInterface|CreateWidget 0))
  (bind _output_get (Variables|Default|SetREF_UI_Collectable 0 _returnvalue))
  (UserInterface|Viewport|AddtoViewport _output_get 0)
  (Rendering|Components|TextRender|SetText (Variables|Default|GetCollected (.REF_UI_Collectable (Variables|Default|GetREF_UI_Collectable))) (Utilities|Text|ToText(String) (Utilities|String|Append "Vous avez reçu : " (Utilities|String|ToString(Float) (Variables|Default|GetBattery%20To%20Add)) " %")))
  (Default|GetBattery _asfirst_person_character (Variables|Default|GetBattery%20To%20Add) _output_get)
  (Actor|DestroyActor))

(event EventBeginPlay)

(fn ConstructionScript)