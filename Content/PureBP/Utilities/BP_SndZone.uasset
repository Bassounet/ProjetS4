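; BP_SndZone is a trigger zone that plays a sound the first time the first-person character enters its box.
; On overlap it plays the configured sound either in 2D or at a set location with attenuation, depending on a flag.
; A Played flag is set afterward, so the zone fires only once.
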(event OnComponentBeginOverlap(Box)
  (params (OverlappedComponent :type Primitive%20Component%20Object%20Reference) (OtherActor :type Actor%20Object%20Reference) (OtherComp :type Primitive%20Component%20Object%20Reference) (OtherBodyIndex :type Integer) (bFromSweep :type Boolean) (SweepResult :type Hit%20Result%20Structure%20%28by%20ref%29))
  (bind _sound_to_play (Variables|Default|GetSound%20To%20Play))
  ;[1 1 1] Zone Son Interact
  (if (not (Variables|Default|GetPlayed?))
    (Utilities|Casting|CastToFirstPersonCharacter OtherActor)
    (if (Variables|Default|Get2D?)
      (Audio|PlaySound2D _sound_to_play 1.0 1.0 0.0 0 0)
      (else
        (Audio|PlaySoundatLocation _sound_to_play (Variables|Default|GetLocation) "0, 0, 0" 1.0 1.0 0.0 (Variables|Default|GetAttenuation%20Settings) 0 0 0)))
    (Variables|Default|SetPlayed? true)))

(event EventBeginPlay)

(event Collision|EventActorBeginOverlap
  (params (OtherActor :type Actor%20Object%20Reference)))

(event EventTick
  (params (DeltaSeconds :type Float%20%28single-precision%29)))

(fn ConstructionScript)