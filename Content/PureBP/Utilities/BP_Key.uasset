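; BP_Key is a pickup key that the player collects by interacting with it.
; Interact sets GotKey on the player character, plays a pickup sound, restores the main cursor, destroys the actor and shows the Key icon on the main HUD.
; Cursored and UnCursored toggle the HUD hand cursor, guarded by a LookAtMe flag on entry.
; An OutlineDetection overlap toggles a highlight on the key mesh.
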(event OnComponentBeginOverlap(OutlineDetection)
  (params (OverlappedComponent :type Primitive%20Component%20Object%20Reference) (OtherActor :type Actor%20Object%20Reference) (OtherComp :type Primitive%20Component%20Object%20Reference) (OtherBodyIndex :type Integer) (bFromSweep :type Boolean) (SweepResult :type Hit%20Result%20Structure%20%28by%20ref%29))
  ;[1 1 1] Overlapp Activate Highlight
  (CallFunction|EnableHighlight (Variables|Default|GetKeyMesh)))

(event OnComponentEndOverlap(OutlineDetection)
  (params (OverlappedComponent :type Primitive%20Component%20Object%20Reference) (OtherActor :type Actor%20Object%20Reference) (OtherComp :type Primitive%20Component%20Object%20Reference) (OtherBodyIndex :type Integer))
  ;[1 1 1] Overlapp Activate Highlight
  (CallFunction|DisableHighlight (Variables|Default|GetKeyMesh)))

(event Custom|DisappearHandCursor
  (bind _as_first_person_character (Variables|Default|GetAs%20First%20Person%20Character))
  (bind _ref_mainhud (Variables|/Game/PureBP/Player/FirstPersonCharacter.FirstPersonCharacter_C|GetREF_MainHud _as_first_person_character))
  ;[1 1 1] Cursor Event
  (Widget|SetVisibility (Variables|/Game/PureBP/UI/BP/W_MainHud.W_MainHud_C|GetPrincipalCursor _ref_mainhud) "Visible")
  (Widget|SetVisibility (Variables|/Game/PureBP/UI/BP/W_MainHud.W_MainHud_C|GetHand _ref_mainhud) "Hidden"))

(event EventUnCursored
  ;[1 1 1] Cursor Event
  (CallFunction|AppearCursor)
  (Widget|SetVisibility (Variables|/Game/PureBP/UI/BP/W_MainHud.W_MainHud_C|GetHand (Variables|/Game/PureBP/Player/FirstPersonCharacter.FirstPersonCharacter_C|GetREF_MainHud (Variables|Default|GetAs%20First%20Person%20Character))) "Hidden")
  (Variables|Default|SetLookAtMe? false))

(event EventCursored
  ;[1 1 1] Cursor Event
  (if (not (Variables|Default|GetLookAtMe?))
    (CallFunction|DesappearCursor)
    (Widget|SetVisibility (Variables|/Game/PureBP/UI/BP/W_MainHud.W_MainHud_C|GetHand (Variables|/Game/PureBP/Player/FirstPersonCharacter.FirstPersonCharacter_C|GetREF_MainHud (Variables|Default|GetAs%20First%20Person%20Character))) "Visible")
    (Variables|Default|SetLookAtMe? true)))

(event EventInteract
  ;[1 1 1] Interact
  (bind _asfirst_person_character (CallFunction|GetPlayer))
  (bind _output_get (Variables|Default|SetCharacterRef _asfirst_person_character))
  (Variables|/Game/PureBP/Player/FirstPersonCharacter.FirstPersonCharacter_C|SetGotKey? _output_get true)
  (Audio|PlaySound2D "/Engine/VREditor/Sounds/UI/Object_PickUp.Object_PickUp" 5.0 1.0 0.0 0 0)
  (CallFunction|DisappearHandCursor)
  (Actor|DestroyActor)
  (bind _ref_mainhud (CallFunction|GetHUD))
  (bind _output_get_2 (Variables|Default|SetREF%20Main%20Hud _ref_mainhud))
  (Widget|SetVisibility (Variables|/Game/PureBP/UI/BP/W_MainHud.W_MainHud_C|GetKey _output_get_2) "Visible"))

(event EventBeginPlay
  ;[1 1 1] récup du hud
  (bind _asfirst_person_character (CallFunction|GetPlayer))
  (Variables|Default|SetAs%20First%20Person%20Character _asfirst_person_character))

(fn ConstructionScript)