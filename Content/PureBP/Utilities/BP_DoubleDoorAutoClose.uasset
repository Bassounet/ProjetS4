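; One-shot double door that the player opens and that later shuts automatically behind a trigger.
; Cursor focus within the Front overlap shows a W_DoorInteract prompt, enabling Interact to swing both leaves open via timeline yaw lerps.
; The player entering Box reverses the swing once, then plays a closing sound and a delayed 2D clip.
; Key-lock prompt logic exists, but hard-coded branch conditions bypass it.
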(event OnComponentBeginOverlap(Front)
  (params (OverlappedComponent :type Primitive%20Component%20Object%20Reference) (OtherActor :type Actor%20Object%20Reference) (OtherComp :type Primitive%20Component%20Object%20Reference) (OtherBodyIndex :type Integer) (bFromSweep :type Boolean) (SweepResult :type Hit%20Result%20Structure%20%28by%20ref%29))
  ;[1 1 1] FRONT
  (Utilities|Casting|CastToBoxComponent OtherComp
    (:CastFailed
      (Utilities|Casting|CastToSphereComponent OtherComp
        (:CastFailed
          (bind _asfirst_person_character (Utilities|Casting|CastToFirstPersonCharacter OtherActor))
          (Variables|Default|SetREF%20First%20Person%20Character _asfirst_person_character)
          (Variables|Default|SetInRange true))))))

(event OnComponentEndOverlap(Front)
  (params (OverlappedComponent :type Primitive%20Component%20Object%20Reference) (OtherActor :type Actor%20Object%20Reference) (OtherComp :type Primitive%20Component%20Object%20Reference) (OtherBodyIndex :type Integer))
  ;[1 1 1] FRONT
  (Utilities|Casting|CastToBoxComponent OtherComp
    (:CastFailed
      (Utilities|Casting|CastToSphereComponent OtherComp
        (:CastFailed
          (Utilities|Casting|CastToFirstPersonCharacter OtherActor)
          (Variables|Default|SetInRange false))))))

(event OnComponentBeginOverlap(Box)
  (params (OverlappedComponent :type Primitive%20Component%20Object%20Reference) (OtherActor :type Actor%20Object%20Reference) (OtherComp :type Primitive%20Component%20Object%20Reference) (OtherBodyIndex :type Integer) (bFromSweep :type Boolean) (SweepResult :type Hit%20Result%20Structure%20%28by%20ref%29))
  (Utilities|Casting|CastToFirstPersonCharacter OtherActor)
  (if (not (Variables|Default|GetHasBeenClosed?))
    (Variables|Default|SetHasBeenClosed? true)
    (bind _openthedoor (Timeline|Timeline_0 Play)
      (:Update
        (Transformation|SetRelativeRotation (Variables|Default|GetR_Door) (Math|Rotator|MakeRotator 0.0 0.0 (Math|Float|Lerp 9e+01 0.0 _openthedoor)) false false)
        (Transformation|SetRelativeRotation (Variables|Default|GetL_Door) (Math|Rotator|MakeRotator 0.0 0.0 (Math|Float|Lerp -9e+01 0.0 _openthedoor)) false false))
      (:Finished
        (Audio|PlaySoundatLocation "/Game/SND/Bank/Door/SC_Door_AutoClose.SC_Door_AutoClose" (Transformation|GetActorLocation) "0, 0, 0" 1.0 1.0 0.0 0 0 0 0)
        (Utilities|FlowControl|Delay 1.0)
        (Audio|PlaySound2D "/Game/SND/Bank/Doublages_Féminins/9_Salle5/SC_PortesReferment_Orianne.SC_PortesReferment_Orianne" 1.0 1.0 0.0 0 0)))))

(event Custom|InteractDoor
  ;[1 1 1] Moving Door Interaction
  (if (not (Variables|Default|GetHasBeenOpened?))
    (Variables|Default|SetHasBeenOpened? true)
    (if (Variables|Default|GetInRange)
      (Audio|PlaySoundatLocation "/Game/SND/Bank/Door/SC_DoorOpen.SC_DoorOpen" (Transformation|GetActorLocation) "0, 0, 0" 1.0 1.0 0.0 0 0 0 0)
      (bind _openthedoor (Timeline|TimeOpenDoor Play)
        (:Update
          (Transformation|SetRelativeRotation (Variables|Default|GetR_Door) (Math|Rotator|MakeRotator 0.0 0.0 (Math|Float|Lerp 0.0 9e+01 _openthedoor)) false false)
          (Transformation|SetRelativeRotation (Variables|Default|GetL_Door) (Math|Rotator|MakeRotator 0.0 0.0 (Math|Float|Lerp 0.0 -9e+01 _openthedoor)) false false))))))

(event Custom|WichHud
  ;[1 1 1] WICH HUD
  (if (not (Variables|Default|GetHasBeenOpened?))
    (CallFunction|HudOpenDoor)))

(event Custom|HudOpenDoor
  ;[1 1 1] Choose HUD
  (if (not false)
    (Variables|Default|SetInteractable? true :!label _label)
    (Default|AppearDoorInteract (Variables|Default|GetREF_HudDoor) "[F] To Open Door" "Hidden" "Visible")
    (Variables|Default|SetAldyCreated? true)
    (elif (not false)
      (goto _label)
      (elif (Variables|/Game/PureBP/Player/FirstPersonCharacter.FirstPersonCharacter_C|GetGotKey? (Variables|Default|GetREF%20First%20Person%20Character))
        (goto _label)
        (else
          (Variables|Default|SetInteractable? false)
          (Default|AppearDoorInteract (Variables|Default|GetREF_HudDoor) "Vous avez besoin de la clef" "Visible" "Hidden")
          (Variables|Default|SetAldyCreated? true))))))

(event EventUnCursored
  ;[1 1 1] Get Cursor
  (Default|DesappearDoorInteract (Variables|Default|GetREF_HudDoor))
  (Variables|Default|SetInteractable? false)
  (Variables|Default|SetAldyCreated? false))

(event EventCursored
  ;[1 1 1] Get Cursor
  (if (Variables|Default|GetInRange)
    (if (not (Variables|Default|GetAldyCreated?))
      (CallFunction|WichHud))))

(event EventBeginPlay
  ;[1 1 1] GET REF
  (bind _returnvalue (UserInterface|CreateWidget "/Game/PureBP/UI/BP/W_DoorInteract.W_DoorInteract_C"))
  (bind _output_get (Variables|Default|SetREF_HudDoor _returnvalue))
  (UserInterface|Viewport|AddtoViewport _output_get 0)
  (if true
    _))

(event EventInteract
  ;[1 1 1] Comment
  ;;[1 1 1] Comment
  (if (Variables|Default|GetInteractable?)
    (CallFunction|InteractDoor)
    (elif true
      (Development|PrintString "La porte est bloquée par la clef")
      (else
        (Development|PrintString "Tu ne peux pas interagir avec la tepor")))))

(fn ConstructionScript)