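; BP_Neon is a neon light actor with two rect lights that can stay intact or flicker, chosen by its Selection setting.
; The construction script applies the light color, and for Intact makes both lights static at LightIntensity.
; On BeginPlay, Full Clignotage continuously runs a timeline toward random intensities.
; Semi Clignotage alternates timer-driven flicker bursts with random pauses, also using a timeline to lerp intensity.
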(event Custom|SemiClignot
  ;[1 1 1] Semi Clignoatge
  ;;[1 1 1] Comment
  (bind _returnvalue (Utilities|Time|SetTimerbyEvent (delegate Custom|CustomEvent_1) (Math|Random|RandomFloatinRange 0.01 0.4) true :!label _label))
  (Variables|Default|SetRef_Timer _returnvalue)
  (Utilities|FlowControl|Delay (Math|Random|RandomFloatinRange 1.0 2.0))
  (Utilities|Time|ClearandInvalidateTimerbyHandle (Variables|Default|GetRef_Timer))
  (Utilities|FlowControl|Delay (Math|Random|RandomFloatinRange 2.0 3.0))
  (goto _label))

(event Custom|CustomEvent_1
  ;[1 1 1] Semi Clignoatge
  (Variables|Default|SetMawLight (Math|Random|RandomFloatinRange (/ (Variables|Default|GetLightIntensity) 5.0) (Variables|Default|GetLightIntensity)))
  (bind _newtrack_0 (Timeline|Timeline_2 Play)
    (:Update
      (Rendering|Components|Light|SetIntensity (Variables|Default|GetRectLight) (Math|Float|Lerp (+ (Variables|/Script/Engine.LightComponentBase|GetIntensity (Variables|Default|GetRectLight)) (Variables|/Script/Engine.LightComponentBase|GetIntensity (Variables|Default|GetRectLight1))) (Variables|Default|GetMawLight) _newtrack_0)))))

(event Custom|Clignotage
  ;[1 1 1] Full Clignotage
  (Utilities|FlowControl|RetriggerableDelay (Math|Random|RandomFloatinRange 0.1 0.09) :!label _label)
  (Variables|Default|SetMawLight (Math|Random|RandomFloatinRange (/ (Variables|Default|GetLightIntensity) 3.0) (Variables|Default|GetLightIntensity)))
  (bind _newtrack_0 (Timeline|Timeline_0 Play)
    (:Update
      (Rendering|Components|Light|SetIntensity (Variables|Default|GetRectLight) (Math|Float|Lerp (+ (Variables|/Script/Engine.LightComponentBase|GetIntensity (Variables|Default|GetRectLight)) (Variables|/Script/Engine.LightComponentBase|GetIntensity (Variables|Default|GetRectLight1))) (Variables|Default|GetMawLight) _newtrack_0)))
    (:Finished
      (Components|Timeline|SetPlayRate (Variables|Default|GetTimeline_0) (/ 1.0 (Variables|Default|GetDuration)))
      (goto _label))))

(event EventBeginPlay
  (switch Utilities|FlowControl|Switch|SwitchonEN_ModeClignotage (Variables|Default|GetSelection)
    (:NewEnumerator0
      (CallFunction|Clignotage))
    (:NewEnumerator1
      (CallFunction|SemiClignot))))

(event Collision|EventActorBeginOverlap
  (params (OtherActor :type Actor%20Object%20Reference)))

(event EventTick
  (params (DeltaSeconds :type Float%20%28single-precision%29)))

(fn ConstructionScript
  (bind _lightintensity (Variables|Default|GetLightIntensity))
  (Rendering|Components|Light|SetLightColor (Variables|Default|GetRectLight1) (Variables|Default|GetNew%20Light%20Color) true)
  (switch Utilities|FlowControl|Switch|SwitchonEN_ModeClignotage (Variables|Default|GetSelection)
    (:NewEnumerator2
      (Transformation|SetMobility (Variables|Default|GetRectLight) "Static")
      (Rendering|Components|Light|SetIntensity (Variables|Default|GetRectLight1) _lightintensity)
      (Rendering|Components|Light|SetIntensity (Variables|Default|GetRectLight) _lightintensity))))