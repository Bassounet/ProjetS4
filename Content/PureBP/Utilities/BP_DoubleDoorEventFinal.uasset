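; Final-event double door: a box overlap shows an interact prompt, and Interact triggers a one-time ending cutscene before loading Test_Concept.
; Interact disables player input and light, blends to a cine camera and plays the CineEventFinal sequence.
; A timeline swings both doors open, with delays chained off its update to reset them and play a gender-specific voice cue.
; The branch restoring camera, input, light and HUD is unconnected.
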(event OnComponentEndOverlap(Box)
  (params (OverlappedComponent :type Primitive%20Component%20Object%20Reference) (OtherActor :type Actor%20Object%20Reference) (OtherComp :type Primitive%20Component%20Object%20Reference) (OtherBodyIndex :type Integer))
  ;[0 1 0.1551] BOX
  (Utilities|Casting|CastToFirstPersonCharacter OtherActor)
  (Variables|Default|SetcanOpenDoor false)
  (Default|DesappearDoorInteract (Variables|Default|GetREF_HudDoor)))

(event OnComponentBeginOverlap(Box)
  (params (OverlappedComponent :type Primitive%20Component%20Object%20Reference) (OtherActor :type Actor%20Object%20Reference) (OtherComp :type Primitive%20Component%20Object%20Reference) (OtherBodyIndex :type Integer) (bFromSweep :type Boolean) (SweepResult :type Hit%20Result%20Structure%20%28by%20ref%29))
  ;[0 0.4072 0.06301] BOX
  (Utilities|Casting|CastToFirstPersonCharacter OtherActor)
  (Variables|Default|SetcanOpenDoor true)
  (CallFunction|HudOpenDoor))

(event Custom|HudOpenDoor
  ;[1 1 1] Comment
  (Default|AppearDoorInteract (Variables|Default|GetREF_HudDoor) "To Open Door" "Hidden" "Visible" "Hidden"))

(event EventInteract
  (bind _returnvalue (Game|GetPlayerController 0))
  ;[1 0.772 0] BiG EvenT
  (if (Variables|Default|GetcanOpenDoor)
    (if (not (Variables|Default|GetHasBeenClosed?))
      (Variables|Default|SetHasBeenClosed? true)
      (Widget|SetVisibility (Variables|Default|GetREF_HudDoor) "Hidden")
      (Input|DisableInput (Game|GetPlayerCharacter 0) _returnvalue)
      (Variables|Default|SetPlayer%20camera (Pawn|GetViewTarget (Game|GetPlayerController 0)))
      (Game|Player|SetViewTargetwithBlend _returnvalue (Components|GetOwner (Variables|Default|GetCineCamera)) 1.0 "VTBlend_Linear" 0.0 false)
      (bind _returnvalue_2 (Sequencer|Player|CreateLevelSequencePlayer "/Game/Cinematics/Sequences/Sequence/CineEventFinal.CineEventFinal"))
      (Sequencer|Player|Play _returnvalue_2 :!class /Script/MovieScene.MovieSceneSequencePlayer)
      (bind _returnvalue_3 (Actor|GetActorOfClass "/Game/PureBP/Player/FirstPersonCharacter.FirstPersonCharacter_C"))
      (Default|DisableLight _returnvalue_3)
      (bind _openthedoor (Timeline|Timeline_0 PlayFromStart)
        (:Update
          (Transformation|SetRelativeRotation (Variables|Default|GetR_Door) (Math|Rotator|MakeRotator 0.0 0.0 (Math|Float|Lerp 0.0 9e+01 _openthedoor)) false false)
          (Transformation|SetRelativeRotation (Variables|Default|GetL_Door) (Math|Rotator|MakeRotator 0.0 0.0 (Math|Float|Lerp 0.0 -9e+01 _openthedoor)) false false)
          (Utilities|FlowControl|Delay 1.0)
          (Transformation|SetRelativeRotation (Variables|Default|GetR_Door) (Math|Rotator|MakeRotator 0.0 0.0 0.0) false false)
          (Transformation|SetRelativeRotation (Variables|Default|GetL_Door) (Math|Rotator|MakeRotator 0.0 0.0 0.0) false false)
          (Utilities|FlowControl|Delay 12.0)
          (bind _asbp_gi (CallFunction|GetBPGI))
          (switch Utilities|FlowControl|Switch|SwitchonEN_MaleFemaleVoice (Variables|/Game/PureBP/BP_GI.BP_GI_C|GetMaleFemale _asbp_gi)
            (:NewEnumerator0
              (Audio|PlaySound2D "/Game/SND/Bank/Doublages_Masculins/CinematiqueFin/SC_Jade_CinematiqueFin.SC_Jade_CinematiqueFin" 1.0 1.0 0.0 0 0))
            (:NewEnumerator1
              (Audio|PlaySound2D "/Game/SND/Bank/Doublages_Féminins/CinematiqueFin/SC_Orianne_CinematiqueFin.SC_Orianne_CinematiqueFin" 1.0 1.0 0.0 0 0))))
        (:Finished
          (Audio|PlaySoundatLocation "/Game/SND/Bank/Door/SC_Door_AutoClose.SC_Door_AutoClose" (Transformation|GetActorLocation) "0, 0, 0" 1.0 1.0 0.0 0 0 0 0)
          (Utilities|FlowControl|Delay (Class|TimeManagementBlueprintLibrary|ToSeconds(QualifiedFrameTime) (Media|MediaPlayer|GetDuration _returnvalue_2)))
          (Game|OpenLevel(byName) "Test_Concept"))))))

(event EventBeginPlay
  ;[1 1 1] GET REF
  (bind _returnvalue (UserInterface|CreateWidget "/Game/PureBP/UI/BP/W_DoorInteract.W_DoorInteract_C"))
  (bind _output_get (Variables|Default|SetREF_HudDoor _returnvalue))
  (UserInterface|Viewport|AddtoViewport _output_get 0))

(fn ConstructionScript)