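; BP_Light is a light actor with three spotlights that share a configurable color and can optionally flicker.
; BeginPlay applies the color and, if Clignote is set, starts the Clignotage event.
; That event waits briefly, picks a random target intensity, and uses a timeline to lerp all three lights from SpotLight2's current intensity toward it.
; On finish, it sets the play rate from Duration and loops back.
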(event Custom|Clignotage
  (Utilities|FlowControl|RetriggerableDelay (Math|Random|RandomFloatinRange 0.1 0.09) :!label _label)
  (Variables|Default|SetMaxLight (Math|Random|RandomFloatinRange 0.0 1e+04))
  (bind _newtrack_0 (Timeline|Timeline_0 Play)
    (:Update
      (Rendering|Components|Light|SetIntensity (Variables|Default|GetSpotLight1) (Math|Float|Lerp (Variables|/Script/Engine.LightComponentBase|GetIntensity (Variables|Default|GetSpotLight2)) (Variables|Default|GetMaxLight) _newtrack_0)))
    (:Finished
      (Components|Timeline|SetPlayRate (Variables|Default|GetTimeline_0) (/ 1.0 (Variables|Default|GetDuration)))
      (goto _label))))

(event EventBeginPlay
  (Rendering|Components|Light|SetLightColor (Variables|Default|GetSpotLight2) (Variables|Default|GetNew%20Light%20Color) true)
  (if (Variables|Default|GetClignote?)
    (CallFunction|Clignotage)))

(event Collision|EventActorBeginOverlap
  (params (OtherActor :type Actor%20Object%20Reference)))

(event EventTick
  (params (DeltaSeconds :type Float%20%28single-precision%29)))

(fn ConstructionScript)