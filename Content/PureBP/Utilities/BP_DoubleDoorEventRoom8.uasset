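; One-shot double door event for Room 8 that plays an entrance cinematic when the player opens it.
; A box overlap shows or hides the interact prompt and gates Interact, which disables input, blends to the cine camera, plays the CineEnteringRoom8 sequence and swings both doors open by timeline.
; A door sound then plays, the player teleports to a hardcoded location, and a short timer restores camera, input and HUD.
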(event OnComponentEndOverlap(Box)
  (params (OverlappedComponent :type Primitive%20Component%20Object%20Reference) (OtherActor :type Actor%20Object%20Reference) (OtherComp :type Primitive%20Component%20Object%20Reference) (OtherBodyIndex :type Integer))
  (Utilities|Casting|CastToFirstPersonCharacter OtherActor)
  (Variables|Default|SetcanOpenDoor false)
  (Default|DesappearDoorInteract (Variables|Default|GetREF_HudDoor)))

(event OnComponentBeginOverlap(Box)
  (params (OverlappedComponent :type Primitive%20Component%20Object%20Reference) (OtherActor :type Actor%20Object%20Reference) (OtherComp :type Primitive%20Component%20Object%20Reference) (OtherBodyIndex :type Integer) (bFromSweep :type Boolean) (SweepResult :type Hit%20Result%20Structure%20%28by%20ref%29))
  (Utilities|Casting|CastToFirstPersonCharacter OtherActor)
  (Variables|Default|SetcanOpenDoor true)
  (CallFunction|HudOpenDoor))

(event Custom|CustomEvent_0
  (Game|Player|SetViewTargetwithBlend (Game|GetPlayerController 0) (Variables|Default|GetPlayer%20camera) 1.0 "VTBlend_Linear" 0.0 false)
  (Input|EnableInput (Game|GetPlayerCharacter 0) (Game|GetPlayerController 0))
  (bind _ref_mainhud (CallFunction|GetHUD))
  (Widget|SetVisibility _ref_mainhud "Visible"))

(event Custom|HudOpenDoor
  (Default|AppearDoorInteract (Variables|Default|GetREF_HudDoor) "[F] To Open Door" "Hidden" "Visible"))

(event EventInteract
  (bind _returnvalue (Game|GetPlayerController 0))
  (if (Variables|Default|GetcanOpenDoor)
    (if (not (Variables|Default|GetHasBeenClosed?))
      (Variables|Default|SetHasBeenClosed? true)
      (Widget|SetVisibility (Variables|Default|GetREF_HudDoor) "Hidden")
      (Input|DisableInput (Game|GetPlayerCharacter 0) _returnvalue)
      (Variables|Default|SetPlayer%20camera (Pawn|GetViewTarget (Game|GetPlayerController 0)))
      (Game|Player|SetViewTargetwithBlend _returnvalue (Components|GetOwner (Variables|Default|GetCineCamera)) 1.0 "VTBlend_Linear" 0.0 false)
      (bind _returnvalue_2 (Sequencer|Player|CreateLevelSequencePlayer "/Game/Cinematics/Sequences/Sequence/CineEnteringRoom8.CineEnteringRoom8"))
      (Sequencer|Player|Play _returnvalue_2 :!class /Script/MovieScene.MovieSceneSequencePlayer)
      (bind _openthedoor (Timeline|Timeline_0 Play)
        (:Update
          (Transformation|SetRelativeRotation (Variables|Default|GetR_Door) (Math|Rotator|MakeRotator 0.0 0.0 (Math|Float|Lerp 0.0 9e+01 _openthedoor)) false false)
          (Transformation|SetRelativeRotation (Variables|Default|GetL_Door) (Math|Rotator|MakeRotator 0.0 0.0 (Math|Float|Lerp 0.0 -9e+01 _openthedoor)) false false))
        (:Finished
          (Audio|PlaySoundatLocation "/Game/SND/Bank/Door/SC_Door_AutoClose.SC_Door_AutoClose" (Transformation|GetActorLocation) "0, 0, 0" 1.0 1.0 0.0 0 0 0 0)
          (Utilities|FlowControl|Delay 2.0)
          (Transformation|SetActorLocation (Game|GetPlayerCharacter 0) "10740.199219,2700.000000,-23.000000" false false)
          (Utilities|Time|SetTimerbyEvent (delegate Custom|CustomEvent_0) 0.5))))))

(event EventBeginPlay
  ;[1 1 1] GET REF
  (bind _returnvalue (UserInterface|CreateWidget "/Game/PureBP/UI/BP/W_DoorInteract.W_DoorInteract_C"))
  (bind _output_get (Variables|Default|SetREF_HudDoor _returnvalue))
  (UserInterface|Viewport|AddtoViewport _output_get 0))

(fn ConstructionScript)