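; BP_Cards is a collectible card actor the first-person player picks up.
; Overlapping HighLightDetect highlights the mesh and caches the player; cursor events toggle pickup eligibility and the HUD hand icon.
; Interacting while eligible increments the player's card count, shows a HUD message, passes the card's identity to SelectionCartes and destroys the actor.
; The construction script applies a dynamic material with a sprite texture selected by NameOfObject.
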(event OnComponentBeginOverlap(HighLightDetect)
  (params (OverlappedComponent :type Primitive%20Component%20Object%20Reference) (OtherActor :type Actor%20Object%20Reference) (OtherComp :type Primitive%20Component%20Object%20Reference) (OtherBodyIndex :type Integer) (bFromSweep :type Boolean) (SweepResult :type Hit%20Result%20Structure%20%28by%20ref%29))
  (bind _asfirst_person_character (Utilities|Casting|CastToFirstPersonCharacter OtherActor))
  (Variables|Default|SetAs%20First%20Person%20Character _asfirst_person_character)
  (CallFunction|EnableHighlight (Variables|Default|GetStaticMesh)))

(event OnComponentEndOverlap(HighLightDetect)
  (params (OverlappedComponent :type Primitive%20Component%20Object%20Reference) (OtherActor :type Actor%20Object%20Reference) (OtherComp :type Primitive%20Component%20Object%20Reference) (OtherBodyIndex :type Integer))
  (Utilities|Casting|CastToFirstPersonCharacter OtherActor)
  (CallFunction|DisableHighlight (Variables|Default|GetStaticMesh)))

(event EventBeginPlay)

(event EventCursored
  (Variables|Default|SetRecupable? true)
  (Widget|SetVisibility (Variables|/Game/PureBP/UI/BP/W_MainHud.W_MainHud_C|GetHand (Variables|/Game/PureBP/Player/FirstPersonCharacter.FirstPersonCharacter_C|GetREF_MainHud (Variables|Default|GetAs%20First%20Person%20Character))) "Visible"))

(event EventInteract
  (if (Variables|Default|GetRecupable?)
    (Math|Integer|IncrementInt (Variables|/Game/PureBP/Player/FirstPersonCharacter.FirstPersonCharacter_C|GetNbCards (Variables|Default|GetAs%20First%20Person%20Character))
      (:%20%20
        (Actor|DestroyActor)
        (Default|RecupCard (Variables|/Game/PureBP/Player/FirstPersonCharacter.FirstPersonCharacter_C|GetREF_MainHud (Variables|Default|GetAs%20First%20Person%20Character)) "Vous avez recup une carte")
        (Widget|SetVisibility (Variables|/Game/PureBP/UI/BP/W_MainHud.W_MainHud_C|GetHand (Variables|/Game/PureBP/Player/FirstPersonCharacter.FirstPersonCharacter_C|GetREF_MainHud (Variables|Default|GetAs%20First%20Person%20Character))) "Hidden")
        (Default|SelectionCartes (Variables|Default|GetAs%20First%20Person%20Character) (Variables|Default|GetQuiEstCe?))))))

(event EventUnCursored
  (Variables|Default|SetRecupable? false)
  (Widget|SetVisibility (Variables|/Game/PureBP/UI/BP/W_MainHud.W_MainHud_C|GetHand (Variables|/Game/PureBP/Player/FirstPersonCharacter.FirstPersonCharacter_C|GetREF_MainHud (Variables|Default|GetAs%20First%20Person%20Character))) "Hidden"))

(fn ConstructionScript
  (bind _returnvalue (Rendering|Material|CreateDynamicMaterialInstance "/Game/Material/MI_Cards.MI_Cards" "None" "None" :!class /Script/Engine.KismetMaterialLibrary))
  (Rendering|Material|SetTextureParameterValue _returnvalue "Sprite" (Utilities|Select :Index (Variables|Default|GetNameOfObject) :NewEnumerator0 "/Game/2D/T_CardGreg.T_CardGreg" :NewEnumerator1 "/Game/2D/T_CardAntoine.T_CardAntoine" :NewEnumerator2 "/Game/2D/T_CardAlexis.T_CardAlexis" :NewEnumerator3 "/Game/2D/T_CardQuentin.T_CardQuentin" :NewEnumerator4 "/Game/2D/T_CardDavid.T_CardDavid" :NewEnumerator5 "/Game/2D/T_CardRomain.T_CardRomain" :NewEnumerator6 "/Game/2D/T_CardPerso.T_CardPerso"))
  (Rendering|Material|SetMaterial (Variables|Default|GetStaticMesh) 0 _returnvalue))