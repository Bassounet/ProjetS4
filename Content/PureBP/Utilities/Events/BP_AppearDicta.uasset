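; BP_AppearDicta is a one-shot trigger zone that shows timed on-screen "Dicta" text with a 2D sound.
; BeginPlay creates and adds its own W_DictaAppear widget to the viewport.
; On the first FirstPersonCharacter overlap, it calls DictaON on the character and passes the text and duration to the widget.
; A timer of that same duration then calls DictaOFF on the character.
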(event OnComponentBeginOverlap(ZoneAppearDicta)
  (params (OverlappedComponent :type Primitive%20Component%20Object%20Reference) (OtherActor :type Actor%20Object%20Reference) (OtherComp :type Primitive%20Component%20Object%20Reference) (OtherBodyIndex :type Integer) (bFromSweep :type Boolean) (SweepResult :type Hit%20Result%20Structure%20%28by%20ref%29))
  (if (not (Variables|Default|GetAppeared?))
    (bind _asfirst_person_character (Utilities|Casting|CastToFirstPersonCharacter OtherActor))
    (Variables|Default|SetREF%20First%20Person%20Character _asfirst_person_character)
    (bind _returnvalue (Utilities|Time|SetTimerbyEvent (delegate Custom|Desappear) (Variables|Default|GetTimeBeforeDesappear)))
    (Variables|Default|SetRefTimer _returnvalue)
    (Default|DictaON (Variables|Default|GetREF%20First%20Person%20Character))
    (Default|AppearText (Variables|Default|GetRefHudDicta) (Variables|Default|GetIn%20Text) (Variables|Default|GetTimeBeforeDesappear))
    (Variables|Default|SetAppeared? true)
    (Audio|PlaySound2D (Variables|Default|GetSoundToPlay) 1.0 1.0 0.0 0 0)))

(event Custom|Desappear
  (Default|DictaOFF (Variables|Default|GetREF%20First%20Person%20Character)))

(event EventBeginPlay
  (bind _returnvalue (UserInterface|CreateWidget "/Game/PureBP/UI/BP/W_DictaAppear.W_DictaAppear_C"))
  (bind _output_get (Variables|Default|SetRefHudDicta _returnvalue))
  (UserInterface|Viewport|AddtoViewport _output_get 0))

(fn ConstructionScript)