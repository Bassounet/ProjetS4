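; BP_LightBlinkMenu is a menu light actor that blinks a point light when its Lighton event fires.
; A timeline track toggles the light's visibility, while a counter tracks how many times the event has fired.
; On every third blink it shows the skeletal mesh of BP_Menu_StepMannikin, then hides it and resets the counter when the timeline finishes.
; BeginPlay is empty, and a randomly delayed self-repeating trigger is left disconnected.
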(event Custom|Light%20on
  (Variables|Default|SetMannikinSpawnat3 (+ (Variables|Default|GetMannikinSpawnat3) 1.0))
  (bind _event (Timeline|Timeline_Light_Blink PlayFromStart)
    (:Update
      (Rendering|SetVisibility (Variables|Default|GetPointLight) (== _event 1.0) false)
      (if (== (Variables|Default|GetMannikinSpawnat3) 3.0)
        (bind _returnvalue (Actor|GetActorOfClass "/Game/Level/Antoine/BP_Menu_StepMannikin.BP_Menu_StepMannikin_C"))
        (Rendering|SetVisibility (Variables|/Game/Level/Antoine/BP_Menu_StepMannikin.BP_Menu_StepMannikin_C|GetSkeletalMesh _returnvalue) true false)))
    (:Finished
      (if (== (Variables|Default|GetMannikinSpawnat3) 3.0)
        (bind _returnvalue_2 (Actor|GetActorOfClass "/Game/Level/Antoine/BP_Menu_StepMannikin.BP_Menu_StepMannikin_C"))
        (Rendering|SetVisibility (Variables|/Game/Level/Antoine/BP_Menu_StepMannikin.BP_Menu_StepMannikin_C|GetSkeletalMesh _returnvalue_2) false false)
        (Variables|Default|SetMannikinSpawnat3 0.0)))))

(event EventBeginPlay)

(fn ConstructionScript)