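; BP_SndZone is a one-shot trigger zone that plays a voice or sound clip with on-screen text when the player enters.
; BeginPlay adds a WP_LoreObject widget to the viewport.
; The first FirstPersonCharacter overlap picks male or female text and sound from the game instance's MaleFemale setting, attaching audio to the camera.
; The text disappears after a delay taken from GetAudioTimeSeconds, the world audio clock rather than clip length.
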(event OnComponentBeginOverlap(Box)
  (params (OverlappedComponent :type Primitive%20Component%20Object%20Reference) (OtherActor :type Actor%20Object%20Reference) (OtherComp :type Primitive%20Component%20Object%20Reference) (OtherBodyIndex :type Integer) (bFromSweep :type Boolean) (SweepResult :type Hit%20Result%20Structure%20%28by%20ref%29))
  (bind _hud_loreobject_ref (Variables|Default|GetHUD_LoreObject_REF))
  ;[1 1 1] Zone Son Interact
  (if (not (Variables|Default|GetPlayed?))
    (bind _asfirst_person_character (Utilities|Casting|CastToFirstPersonCharacter OtherActor))
    (Variables|Default|SetAs%20First%20Person%20Character _asfirst_person_character)
    (bind _asbp_gi (CallFunction|GetBPGI))
    (switch Utilities|FlowControl|Switch|SwitchonEN_MaleFemaleVoice (Variables|/Game/PureBP/BP_GI.BP_GI_C|GetMaleFemale _asbp_gi)
      (:NewEnumerator0
        (Default|Appeartext _hud_loreobject_ref (Variables|Default|GetMaleText))
        (Audio|SpawnSoundAttached (Variables|Default|GetSoundMale) (Variables|/Game/PureBP/Player/FirstPersonCharacter.FirstPersonCharacter_C|GetFirstPersonCamera (Variables|Default|GetAs%20First%20Person%20Character)) "None" "0, 0, 0" "0, 0, 0" "KeepRelativeOffset" false 1.0 1.0 0.0 "/Game/SND/SA_V1.SA_V1" 0))
      (:NewEnumerator1
        (Default|Appeartext _hud_loreobject_ref (Variables|Default|GetFemaleText))
        (Audio|SpawnSoundAttached (Variables|Default|GetSound%20To%20Play) (Variables|/Game/PureBP/Player/FirstPersonCharacter.FirstPersonCharacter_C|GetFirstPersonCamera (Variables|Default|GetAs%20First%20Person%20Character)) "None" "0, 0, 0" "0, 0, 0" "KeepRelativeOffset" false 1.0 1.0 0.0 "/Game/SND/SA_V1.SA_V1" 0)))
    (Variables|Default|SetPlayed? true)
    (Utilities|FlowControl|Delay (Class|GameplayStatics|GetAudioTimeSeconds))
    (Default|Desappear (Variables|Default|GetHUD_LoreObject_REF))))

(event EventBeginPlay
  (bind _returnvalue (UserInterface|CreateWidget "/Game/PureBP/UI/BP/WP_LoreObject.WP_LoreObject_C"))
  (bind _output_get (Variables|Default|SetHUD_LoreObject_REF _returnvalue))
  (UserInterface|Viewport|AddtoViewport _output_get 0))

(fn ConstructionScript)