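; BP_TextZone is a trigger zone that shows a text message on screen while something overlaps its box.
; On BeginPlay it creates a WP_TextZone widget, adds it to the viewport and keeps it hidden.
; Box overlap begin shows the widget and fills its text block with TextToDisplay, and overlap end hides it, with no check on which actor overlaps.
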(event OnComponentBeginOverlap(Box)
  (params (OverlappedComponent :type Primitive%20Component%20Object%20Reference) (OtherActor :type Actor%20Object%20Reference) (OtherComp :type Primitive%20Component%20Object%20Reference) (OtherBodyIndex :type Integer) (bFromSweep :type Boolean) (SweepResult :type Hit%20Result%20Structure%20%28by%20ref%29))
  (bind _reftextzonehud (Variables|Default|GetRefTextZoneHUD))
  (Widget|SetVisibility _reftextzonehud "Visible")
  (Rendering|Components|TextRender|SetText (Variables|/Game/PureBP/UI/BP/WP_TextZone.WP_TextZone_C|GetBlocTexte _reftextzonehud) (Variables|Default|GetTextToDisplay)))

(event OnComponentEndOverlap(Box)
  (params (OverlappedComponent :type Primitive%20Component%20Object%20Reference) (OtherActor :type Actor%20Object%20Reference) (OtherComp :type Primitive%20Component%20Object%20Reference) (OtherBodyIndex :type Integer))
  (Widget|SetVisibility (Variables|Default|GetRefTextZoneHUD) "Hidden"))

(event EventBeginPlay
  ;[1 1 1] GetSomeRef
  (bind _returnvalue (UserInterface|CreateWidget "/Game/PureBP/UI/BP/WP_TextZone.WP_TextZone_C"))
  (Variables|Default|SetRefTextZoneHUD _returnvalue)
  (UserInterface|Viewport|AddtoViewport (Variables|Default|GetRefTextZoneHUD) 0)
  (Widget|SetVisibility (Variables|Default|GetRefTextZoneHUD) "Hidden"))

(fn ConstructionScript)