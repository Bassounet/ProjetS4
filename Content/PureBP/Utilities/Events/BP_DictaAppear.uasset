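; BP_DictaAppear is a one-shot trigger that presents a "Dicta" moment with sound and a timed subtitle when the player enters its box.
; It creates its own W_DictaAppear widget on BeginPlay and adds it to the viewport.
; The first FirstPersonCharacter overlap calls DictaON on the character, shows the subtitle and spawns the attached sound.
; A timer using the same duration as the subtitle later calls DictaOFF.
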(event OnComponentBeginOverlap(Box)
  (params (OverlappedComponent :type Primitive%20Component%20Object%20Reference) (OtherActor :type Actor%20Object%20Reference) (OtherComp :type Primitive%20Component%20Object%20Reference) (OtherBodyIndex :type Integer) (bFromSweep :type Boolean) (SweepResult :type Hit%20Result%20Structure%20%28by%20ref%29))
  (if (not (Variables|Default|GetPlayed?))
    (bind _asfirst_person_character (Utilities|Casting|CastToFirstPersonCharacter OtherActor))
    (Variables|Default|SetREF%20First%20Person%20Character _asfirst_person_character)
    (bind _returnvalue (Utilities|Time|SetTimerbyEvent (delegate Custom|DesappearDicta) (Variables|Default|GetTimeBeforeDesappear)))
    (Variables|Default|SetREF_Timer _returnvalue)
    (Variables|Default|SetPlayed? true)
    (CallFunction|AppearDicta)))

(event Custom|DesappearDicta
  (Default|DictaOFF (Variables|Default|GetREF%20First%20Person%20Character)))

(event Custom|AppearDicta
  (Default|DictaON (Variables|Default|GetREF%20First%20Person%20Character))
  (Default|AppearSubtitle (Variables|Default|GetREF_HudDicta) (Variables|Default|GetText%20To%20Display%20Subtitle) (Variables|Default|GetTimeBeforeDesappear))
  (Audio|SpawnSoundAttached (Variables|Default|GetSoundToPlay) 0 "None" "0, 0, 0" "0, 0, 0" "KeepRelativeOffset" false 1.0 1.0 0.0 0 0))

(event EventBeginPlay
  (bind _returnvalue (UserInterface|CreateWidget "/Game/PureBP/UI/BP/W_DictaAppear.W_DictaAppear_C"))
  (bind _output_get (Variables|Default|SetREF_HudDicta _returnvalue))
  (UserInterface|Viewport|AddtoViewport _output_get 0))

(fn ConstructionScript)