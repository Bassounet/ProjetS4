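; BP_AppearMannikins is a one-shot trigger that makes an actor, presumably a mannequin, briefly appear when the first-person player enters its box.
; The overlap ignores box components, then spawns the configurable class at the AppearZone's location and rotation and plays a sound there.
; A timer destroys the spawned actor after a set delay, and a Spawned flag prevents the event from repeating.
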(event OnComponentBeginOverlap(Box)
  (params (OverlappedComponent :type Primitive%20Component%20Object%20Reference) (OtherActor :type Actor%20Object%20Reference) (OtherComp :type Primitive%20Component%20Object%20Reference) (OtherBodyIndex :type Integer) (bFromSweep :type Boolean) (SweepResult :type Hit%20Result%20Structure%20%28by%20ref%29))
  (bind _appearzone (Variables|Default|GetAppearZone))
  (Utilities|Casting|CastToBoxComponent OtherComp
    (:CastFailed
      (Utilities|Casting|CastToFirstPersonCharacter OtherActor)
      (if (not (Variables|Default|GetSpawned?))
        (bind _returnvalue (Game|SpawnActorfromClass (Variables|Default|GetClassToAppear) (Math|Transform|MakeTransform (Transformation|GetWorldLocation _appearzone) (Transformation|GetWorldRotation _appearzone) "1.000000,1.000000,1.000000") "Undefined" 0 0))
        (Variables|Default|SetREF_MannikinsAppeared _returnvalue)
        (Audio|PlaySoundatLocation (Variables|Default|GetSoundToPlay) (Transformation|GetWorldLocation (Variables|Default|GetAppearZone)) "0, 0, 0" 1.0 1.0 0.0 "/Game/SND/SA_V1.SA_V1" 0 0 0)
        (Utilities|Time|SetTimerbyEvent (delegate Custom|Desappear) (Variables|Default|GetTimeToWaitBeforeDesappear))
        (Variables|Default|SetSpawned? true)))))

(event Custom|Desappear
  (Actor|DestroyActor (Variables|Default|GetREF_MannikinsAppeared)))

(fn ConstructionScript)