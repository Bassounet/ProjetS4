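; BP_SavePoint is a one-shot checkpoint actor that sets the first-person character's zone respawn transform.
; When the character enters its Box, a Camera-channel trace from the root toward it must report a hit distance within MinimalDistanceForActiv.
; Saving copies the Arrow's location and rotation to the character, plays a sound and sets Saved to block retriggering.
; A W_SavePoint widget, created on BeginPlay, then shows the save logo.
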(event OnComponentBeginOverlap(Box)
  (params (OverlappedComponent :type Primitive%20Component%20Object%20Reference) (OtherActor :type Actor%20Object%20Reference) (OtherComp :type Primitive%20Component%20Object%20Reference) (OtherBodyIndex :type Integer) (bFromSweep :type Boolean) (SweepResult :type Hit%20Result%20Structure%20%28by%20ref%29))
  ;[1 1 1] Interact in/ Out
  (if (not (Variables|Default|GetSaved?))
    (bind _asfirst_person_character (Utilities|Casting|CastToFirstPersonCharacter OtherActor))
    (Variables|Default|SetREF_Fp _asfirst_person_character)
    (bind _outhit (Collision|LineTraceByChannel (Transformation|GetWorldLocation (Variables|Default|GetDefaultSceneRoot)) (Transformation|GetActorLocation OtherActor) "TraceTypeQuery2" false 0 "ForDuration"))
    (if (<= (.Distance (Collision|BreakHitResult _outhit)) (Variables|Default|GetMinimalDistanceForActiv))
      (CallFunction|SavePoint))))

(event Custom|SavePoint
  (bind _arrow (Variables|Default|GetArrow))
  (bind _ref_fp (Variables|Default|GetREF_Fp))
  ;[1 1 1] Save
  (Variables|/Game/PureBP/Player/FirstPersonCharacter.FirstPersonCharacter_C|SetZone%20Respawn%20Location _ref_fp (Transformation|GetWorldLocation _arrow))
  (Variables|/Game/PureBP/Player/FirstPersonCharacter.FirstPersonCharacter_C|SetZone%20Respawn%20Rotation _ref_fp (Transformation|GetWorldRotation _arrow))
  (Audio|PlaySound2D "/Engine/VREditor/Sounds/UI/Click_on_Button_Cue.Click_on_Button_Cue" 1.0 1.0 0.0 0 0)
  (Variables|Default|SetSaved? true)
  (Default|AppearLogoSave (Variables|Default|GetREF_HUDSavePoint)))

(event EventBeginPlay
  ;[1 1 1] Comment
  (bind _returnvalue (UserInterface|CreateWidget "/Game/PureBP/UI/BP/W_SavePoint.W_SavePoint_C"))
  (bind _output_get (Variables|Default|SetREF_HUDSavePoint _returnvalue))
  (UserInterface|Viewport|AddtoViewport _output_get 0))

(fn ConstructionScript)