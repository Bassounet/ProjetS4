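; BP_EventSalle7_EntreeSol is a one-shot audio event for Room 7, driven by the first-person character crossing two trigger boxes.
; The first overlap with BoxEntree spawns the SC_Event_Salle7_EntreeSol 2D sound, stores it and sets Condition to false.
; While Condition is false, the first overlap with BoxSortie fades that stored sound out.
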(event OnComponentBeginOverlap(BoxSortie)
  (params (OverlappedComponent :type Primitive%20Component%20Object%20Reference) (OtherActor :type Actor%20Object%20Reference) (OtherComp :type Primitive%20Component%20Object%20Reference) (OtherBodyIndex :type Integer) (bFromSweep :type Boolean) (SweepResult :type Hit%20Result%20Structure%20%28by%20ref%29))
  (Utilities|Casting|CastToFirstPersonCharacter OtherActor)
  (if (not (Variables|Default|GetCondition))
    (Utilities|FlowControl|DoOnce false
      (:Completed
        (Audio|Components|Audio|FadeOut (Variables|Default|GetSound) 2.0 0.0 "Linear" :!class /Script/Engine.AudioComponent)))))

(event OnComponentBeginOverlap(BoxEntree)
  (params (OverlappedComponent :type Primitive%20Component%20Object%20Reference) (OtherActor :type Actor%20Object%20Reference) (OtherComp :type Primitive%20Component%20Object%20Reference) (OtherBodyIndex :type Integer) (bFromSweep :type Boolean) (SweepResult :type Hit%20Result%20Structure%20%28by%20ref%29))
  (Utilities|Casting|CastToFirstPersonCharacter OtherActor)
  (Utilities|FlowControl|DoOnce false
    (:Completed
      (Variables|Default|SetCondition false)
      (bind _returnvalue (Audio|SpawnSound2D "/Game/SND/Bank/EventsSounds/Event_Salle_7/SC_Event_Salle7_EntreeSol.SC_Event_Salle7_EntreeSol" 1.0 1.0 0.0 0))
      (Variables|Default|SetSound _returnvalue))))

(event EventBeginPlay)

(event Collision|EventActorBeginOverlap
  (params (OtherActor :type Actor%20Object%20Reference)))

(event EventTick
  (params (DeltaSeconds :type Float%20%28single-precision%29)))

(fn ConstructionScript)