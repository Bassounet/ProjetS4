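; Inspectable lore object, static or skeletal mesh, that the player picks up to read its text and hear a gendered voice line.
; Grip attaches it to the character's inspection zone and moves input to the object, so Turn/LookUp rotate it and Interact releases it.
; Gripping also signals a pause through a dispatcher, ducks ambient and FX audio, and shows the lore widget.
; Cursor events toggle a hand icon; proximity overlap toggles highlighting.
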(event OnComponentBeginOverlap(OutlineDetection)
  (params (OverlappedComponent :type Primitive%20Component%20Object%20Reference) (OtherActor :type Actor%20Object%20Reference) (OtherComp :type Primitive%20Component%20Object%20Reference) (OtherBodyIndex :type Integer) (bFromSweep :type Boolean) (SweepResult :type Hit%20Result%20Structure%20%28by%20ref%29))
  ;[1 1 1] HighlightPosition PLayer
  (if (not (Variables|Default|GetGripped?))
    (CallFunction|EnableHighlight (Variables|Default|GetStaticMesh))))

(event OnComponentEndOverlap(OutlineDetection)
  (params (OverlappedComponent :type Primitive%20Component%20Object%20Reference) (OtherActor :type Actor%20Object%20Reference) (OtherComp :type Primitive%20Component%20Object%20Reference) (OtherBodyIndex :type Integer))
  ;[1 1 1] HighlightPosition PLayer
  (if (not (Variables|Default|GetGripped?))
    (CallFunction|DisableHighlight (Variables|Default|GetStaticMesh))))

(event Custom|UnGrip
  (bind _returnvalue (Game|GetPlayerController 0))
  (bind _staticmesh (Variables|Default|GetStaticMesh))
  ;[0 0.01975 1] UnGrip
  (Transformation|DetachFromComponent (Variables|Default|GetDefaultSceneRoot) "KeepWorld" "KeepWorld" "KeepWorld" false)
  (Variables|Default|SetGripped? false)
  (bind _asbp_gi (CallFunction|RecupDispatcher))
  (Default|CallUnPauseAfterRead _asbp_gi)
  (Physics|SetSimulatePhysics _staticmesh true)
  (Collision|SetCollisionEnabled _staticmesh "QueryAndPhysics")
  (Input|DisableInput _returnvalue)
  (Input|EnableInput (Variables|Default|GetREF%20First%20Person%20Character) _returnvalue)
  (CallFunction|EnableHighlight (Variables|Default|GetStaticMesh))
  (Components|Activation|Activate (Variables|Default|GetNiagara) false)
  (CallFunction|ReSoundAmbiance 1.0 0.2)
  (CallFunction|ReSoundFX 1.0 0.2)
  (Default|UnGrab (Variables|Default|GetREF%20First%20Person%20Character))
  (Default|Desappear (Variables|Default|GetREF%20LoreHUD)))

(event Custom|Grip
  (bind _returnvalue (Game|GetPlayerController 0))
  (bind _defaultsceneroot (Variables|Default|GetDefaultSceneRoot))
  (bind _staticmesh (Variables|Default|GetStaticMesh))
  ;[0 1 0.02873] GRIP
  (Transformation|SetRelativeLocationAndRotation (Variables|Default|GetStaticMesh) "0, 0, 0" "0, 0, 0" false false)
  (bind _asfirst_person_character (CallFunction|GetPlayer))
  (Variables|Default|SetREF%20First%20Person%20Character _asfirst_person_character)
  (Variables|Default|SetGripped? true)
  (bind _asbp_gi (CallFunction|RecupDispatcher))
  (Default|CallPausewhenReadLore _asbp_gi)
  (if (Variables|Default|GetSkeletal?)
    (Physics|SetSimulatePhysics (Variables|Default|GetSK_Manikin_Arm) true)
    (Transformation|AttachComponentToComponent _defaultsceneroot (Variables|/Game/PureBP/Player/FirstPersonCharacter.FirstPersonCharacter_C|GetZoneTeleportInspection (Variables|Default|GetREF%20First%20Person%20Character)) "None" "SnapToTarget" "SnapToTarget" "KeepWorld" true)
    (else
      (Physics|SetSimulatePhysics _staticmesh false)
      (Collision|SetCollisionEnabled _staticmesh "NoCollision")
      (Transformation|AttachComponentToComponent _defaultsceneroot (Variables|/Game/PureBP/Player/FirstPersonCharacter.FirstPersonCharacter_C|GetZoneTeleportInspection (Variables|Default|GetREF%20First%20Person%20Character)) "None" "SnapToTarget" "SnapToTarget" "KeepWorld" true)))
  (Input|DisableInput (Variables|Default|GetREF%20First%20Person%20Character) _returnvalue)
  (Input|EnableInput _returnvalue)
  (Default|Appeartext (Variables|Default|GetREF%20LoreHUD) (Variables|Default|Gettext%20to%20display))
  (if (not (Variables|Default|GetSkeletal?))
    (CallFunction|DisableHighlight (Variables|Default|GetStaticMesh))
    (else
      (CallFunction|DisableHighlight (Variables|Default|GetSK_Manikin_Arm))))
  (Components|Activation|Deactivate (Variables|Default|GetNiagara))
  (CallFunction|NoSoundAmbiance 0.2 0.0)
  (Default|GrabObject (Variables|Default|GetREF%20First%20Person%20Character))
  (CallFunction|NoSoundFX 0.0 0.2)
  (switch Utilities|FlowControl|Switch|SwitchonEN_MaleFemaleVoice (Variables|/Game/PureBP/BP_GI.BP_GI_C|GetMaleFemale (Variables|Default|GetBP_GI_Ref))
    (:NewEnumerator0
      (Audio|SpawnSoundAttached (Variables|Default|GetSoundMale) (Components|GetChildComponent (Variables|/Script/Engine.Character|GetCapsuleComponent (Variables|Default|GetREF%20First%20Person%20Character)) 0) "None" (Transformation|GetActorLocation (Variables|Default|GetREF%20First%20Person%20Character)) "0, 0, 0" "KeepRelativeOffset" false 1.0 1.0 0.0 "/Game/SND/SA_V1_2.SA_V1_2" 0))
    (:NewEnumerator1
      (bind _returnvalue_2 (Audio|SpawnSoundAttached (Variables|Default|GetSoundFemale) (Components|GetChildComponent (Variables|/Script/Engine.Character|GetCapsuleComponent (Variables|Default|GetREF%20First%20Person%20Character)) 0) "None" (Transformation|GetActorLocation (Variables|Default|GetREF%20First%20Person%20Character)) "0, 0, 0" "KeepRelativeOffset" false 1.0 1.0 0.0 "/Game/SND/SA_V1_2.SA_V1_2" 0))
      (Variables|Default|SetSoundOfDialogue _returnvalue_2)))
  (Audio|SpawnSoundAttached "/Game/SND/Bank/GrabObjects/SC_GrabObjects.SC_GrabObjects" (Variables|Default|GetStaticMesh) "None" "0, 0, 0" "0, 0, 0" "KeepRelativeOffset" false 1.0 1.0 0.0 "/Game/SND/SA_V1.SA_V1" 0))

(event EventBeginPlay
  ;[1 1 1] Comment
  (bind _returnvalue (UserInterface|CreateWidget "/Game/PureBP/UI/BP/WP_LoreObject.WP_LoreObject_C"))
  (bind _output_get (Variables|Default|SetREF%20LoreHUD _returnvalue))
  (UserInterface|Viewport|AddtoViewport _output_get 0)
  (bind _asbp_gi (CallFunction|GetBPGI))
  (Variables|Default|SetBP_GI_Ref _asbp_gi)
  (if (Variables|Default|GetSkeletal?)
    (Rendering|SetVisibility (Variables|Default|GetStaticMesh) false false)
    (else
      (Rendering|SetVisibility (Variables|Default|GetSK_Manikin_Arm) false false))))

(event EventUnCursored
  ;[0 0 0] Cursor Event
  (Default|DesappearHand (Variables|Default|GetREF%20LoreHUD))
  (Variables|Default|SetLookAtMe? false))

(event EventCursored
  ;[0 0 0] Cursor Event
  (if (not (Variables|Default|GetLookAtMe?))
    (Default|AppearHand (Variables|Default|GetREF%20LoreHUD))
    (Variables|Default|SetLookAtMe? true)))

(event EventInteract
  ;[0.2675 1 0] Gripping
  (if (not (Variables|Default|GetGripped?))
    (CallFunction|Grip)
    (else
      (CallFunction|UnGrip))))

(event Input|ActionEvents|InputActionInteract
  (params (Key :type Key%20Structure :default "None"))
  ;[1 1 1] Comment
  (:Pressed
    (if (Variables|Default|GetGripped?)
      (CallFunction|UnGrip))))

(event Input|AxisEvents|InputAxisTurn
  (params (AxisValue :type Float%20%28single-precision%29))
  ;[1 0.9326 0] Rotate Item
  (Transformation|SetActorRotation (Math|Rotator|CombineRotators (Transformation|GetActorRotation) (Math|Rotator|MakeRotator 0.0 0.0 (* AxisValue -5.0)))))

(event Input|AxisEvents|InputAxisLookUp
  (params (AxisValue :type Float%20%28single-precision%29))
  ;[1 0.9326 0] Rotate Item
  (Transformation|SetActorRotation (Math|Rotator|CombineRotators (Transformation|GetActorRotation) (Math|Rotator|MakeRotator (* AxisValue 5.0) 0.0 0.0))))

(fn ConstructionScript)