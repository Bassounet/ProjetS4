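; BP_DroppingBoxes is a box actor that plays an impact sound when it hits something during a collapse.
; On Hit, it looks up BP_Effondrement and continues only while IsCrumbling is set.
; It plays SC_DroppingBoxes at the hit location, with volume scaled from the mesh's vertical speed and clamped.
; A DoOnce reset after a short Delay throttles repeated sounds.
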(event EventBeginPlay)

(event Collision|EventActorBeginOverlap
  (params (OtherActor :type Actor%20Object%20Reference)))

(event EventTick
  (params (DeltaSeconds :type Float%20%28single-precision%29)))

(event Collision|EventHit
  (params (MyComp :type Primitive%20Component%20Object%20Reference) (Other :type Actor%20Object%20Reference) (OtherComp :type Primitive%20Component%20Object%20Reference) (bSelfMoved :type Boolean) (HitLocation :type Vector :default "0, 0, 0") (HitNormal :type Vector :default "0, 0, 0") (NormalImpulse :type Vector :default "0, 0, 0") (Hit :type Hit%20Result%20Structure%20%28by%20ref%29))
  (bind _returnvalue (Actor|GetActorOfClass "/Game/PureBP/Utilities/Events/BP_Effondrement.BP_Effondrement_C"))
  (if (Variables|/Game/PureBP/Utilities/Events/BP_Effondrement.BP_Effondrement_C|GetIsCrumbling? _returnvalue)
    (Utilities|FlowControl|DoOnce false :!label _label
      (:Completed
        (Audio|PlaySoundatLocation "/Game/SND/Bank/DroppingBoxes/SC_DroppingBoxes.SC_DroppingBoxes" HitLocation "0, 0, 0" (Math|Float|Clamp(Float) (/ (Math|Vector|VectorLength (Math|Conversions|ToVector(Float) (.Z (Math|Vector|BreakVector (Transformation|GetComponentVelocity (Variables|Default|GetStaticMesh)))))) 1.2e+03) 0.0 0.7) 1.0 0.0 0 0 0 0)
        (Utilities|FlowControl|Delay 0.27)
        (goto _label Reset)))))

(fn ConstructionScript)