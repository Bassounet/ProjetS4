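; BP_LightBroken is a one-shot trigger event that breaks the first-person player's torch.
; Entering the box attaches a Niagara effect to the player's light and starts a looping timer, with a randomly chosen interval, that flickers its visibility.
; Leaving activates the effect, stops the timer, hides the light and marks it unusable.
; Both transitions play a low-battery sound on the torch.
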(event OnComponentBeginOverlap(Box)
  (params (OverlappedComponent :type Primitive%20Component%20Object%20Reference) (OtherActor :type Actor%20Object%20Reference) (OtherComp :type Primitive%20Component%20Object%20Reference) (OtherBodyIndex :type Integer) (bFromSweep :type Boolean) (SweepResult :type Hit%20Result%20Structure%20%28by%20ref%29))
  (bind _asfirst_person_character (Utilities|Casting|CastToFirstPersonCharacter OtherActor))
  (bind _output_get (Variables|Default|SetREF%20First%20Person%20Character _asfirst_person_character))
  (Transformation|AttachComponentToComponent (Variables|Default|GetNiagara) (Variables|/Game/PureBP/Player/FirstPersonCharacter.FirstPersonCharacter_C|GetLightLamp _output_get) "None" "KeepRelative" "KeepRelative" "KeepRelative" true)
  (Utilities|FlowControl|DoOnce false
    (:Completed
      (bind _returnvalue (Utilities|Time|SetTimerbyEvent (delegate Custom|CustomEvent_0) (Math|Random|RandomFloatinRange 0.01 0.2) true))
      (Audio|SpawnSoundAttached "/Game/SND/Bank/Lamp/Battery_Low/SC_BatteryLow.SC_BatteryLow" (Variables|/Game/PureBP/Player/FirstPersonCharacter.FirstPersonCharacter_C|GetSM_Torch (Variables|Default|GetREF%20First%20Person%20Character)) "None" "0, 0, 0" "0, 0, 0" "KeepRelativeOffset" false 1.0 1.0 0.0 0 0))))

(event OnComponentEndOverlap(Box)
  (params (OverlappedComponent :type Primitive%20Component%20Object%20Reference) (OtherActor :type Actor%20Object%20Reference) (OtherComp :type Primitive%20Component%20Object%20Reference) (OtherBodyIndex :type Integer))
  (Utilities|Casting|CastToFirstPersonCharacter OtherActor)
  (Utilities|FlowControl|DoOnce false
    (:Completed
      (Components|Activation|Activate (Variables|Default|GetNiagara) false)
      (Rendering|SetVisibility (Variables|/Game/PureBP/Player/FirstPersonCharacter.FirstPersonCharacter_C|GetLightLamp (Variables|Default|GetREF%20First%20Person%20Character)) false false)
      (Variables|/Game/PureBP/Player/FirstPersonCharacter.FirstPersonCharacter_C|SetUsableLight (Variables|Default|GetREF%20First%20Person%20Character) false)
      (Utilities|Time|ClearandInvalidateTimerbyHandle (stale OnComponentBeginOverlap(Box) _returnvalue))
      (Audio|SpawnSoundAttached "/Game/SND/Bank/Lamp/Battery_Low/SC_BatteryLow.SC_BatteryLow" (Variables|/Game/PureBP/Player/FirstPersonCharacter.FirstPersonCharacter_C|GetSM_Torch (Variables|Default|GetREF%20First%20Person%20Character)) "None" "0, 0, 0" "0, 0, 0" "KeepRelativeOffset" false 1.0 1.0 0.0 0 0))))

(event Custom|CustomEvent_0
  (Rendering|ToggleVisibility (Variables|/Game/PureBP/Player/FirstPersonCharacter.FirstPersonCharacter_C|GetLightLamp (Variables|Default|GetREF%20First%20Person%20Character)) false))

(event EventBeginPlay)

(event Collision|EventActorBeginOverlap
  (params (OtherActor :type Actor%20Object%20Reference)))

(event EventTick
  (params (DeltaSeconds :type Float%20%28single-precision%29)))

(fn ConstructionScript)