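; BP_Effondrement2 is a one-shot scripted collapse event that blocks a passage when the FirstPersonCharacter enters its box trigger.
; It enters cinematic mode via the game instance, blends to a cine camera and plays a level sequence, with timers spawning a crate and ending the cutscene.
; After a delay it destroys a cube and plays a gender-specific voice line with subtitles.
; The end timer restores the player camera, enables wall collision and exits cinematic mode.
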(event OnComponentBeginOverlap(Box)
  (params (OverlappedComponent :type Primitive%20Component%20Object%20Reference) (OtherActor :type Actor%20Object%20Reference) (OtherComp :type Primitive%20Component%20Object%20Reference) (OtherBodyIndex :type Integer) (bFromSweep :type Boolean) (SweepResult :type Hit%20Result%20Structure%20%28by%20ref%29))
  (bind _returnvalue (Game|GetPlayerController 0))
  (bind _asfirst_person_character (Utilities|Casting|CastToFirstPersonCharacter OtherActor))
  (Variables|Default|SetAs%20First%20Person%20Character _asfirst_person_character)
  (if (not (Variables|Default|GetIsCrumbling?))
    (Variables|Default|SetIsCrumbling? true)
    (bind _asbp_gi (CallFunction|GetBPGI))
    (bind _output_get (Variables|Default|SetAs%20BP%20GI _asbp_gi))
    (Default|CallCinematic _output_get)
    (Variables|Default|SetPlayerCamera (Pawn|GetViewTarget _returnvalue))
    (Game|Player|SetViewTargetwithBlend _returnvalue (Components|GetOwner (Variables|Default|GetCineCamera)) 1.0 "VTBlend_Linear" 0.0 false)
    (bind _returnvalue_2 (Sequencer|Player|CreateLevelSequencePlayer "/Game/Cinematics/Sequences/Sequence/EventPassageBloque.EventPassageBloque"))
    (Sequencer|Player|Play _returnvalue_2 :!class /Script/MovieScene.MovieSceneSequencePlayer)
    (Utilities|Time|SetTimerbyEvent (delegate Custom|CustomEvent_1) (Class|TimeManagementBlueprintLibrary|ToSeconds(QualifiedFrameTime) (Media|MediaPlayer|GetDuration _returnvalue_2)))
    (Utilities|Time|SetTimerbyEvent (delegate Custom|CustomEvent_0) 1.5)
    (Utilities|FlowControl|Delay 2.8)
    (Components|DestroyComponent (Variables|Default|GetCube))
    (bind _hud_subtitles_ref (CallFunction|GetSubtitlesHUD))
    (switch Utilities|FlowControl|Switch|SwitchonEN_MaleFemaleVoice (Variables|/Game/PureBP/BP_GI.BP_GI_C|GetMaleFemale (Variables|Default|GetAs%20BP%20GI))
      (:NewEnumerator0
        (Audio|SpawnSoundAttached "/Game/SND/Bank/Doublages_Masculins/6_Salle3_PassageBloque/SC_Jade_PassageBloque_Room3.SC_Jade_PassageBloque_Room3" (Variables|/Game/PureBP/Player/FirstPersonCharacter.FirstPersonCharacter_C|GetFirstPersonCamera (Variables|Default|GetAs%20First%20Person%20Character)) "None" "0, 0, 0" "0, 0, 0" "KeepRelativeOffset" false 1.0 1.0 0.0 "/Game/SND/SA_V1.SA_V1" 0)
        (Utilities|FlowControl|Delay 1.5)
        (Default|ChangeSubtitles _hud_subtitles_ref (Variables|Default|GetMaleTextEffondrement) 5.0))
      (:NewEnumerator1
        (Audio|SpawnSoundAttached "/Game/SND/Bank/Doublages_Féminins/6_Salle3_PassageBloque/SC_PassageBloque_orianne.SC_PassageBloque_orianne" (Variables|/Game/PureBP/Player/FirstPersonCharacter.FirstPersonCharacter_C|GetFirstPersonCamera (Variables|Default|GetAs%20First%20Person%20Character)) "None" "0, 0, 0" "0, 0, 0" "KeepRelativeOffset" false 1.0 1.0 0.0 0 0)
        (Utilities|FlowControl|Delay 1.0)
        (Default|ChangeSubtitles _hud_subtitles_ref (Variables|Default|GetFemaleTextEffondrement) 5.0)))))

(event Custom|CustomEvent_0
  (Game|SpawnActorfromClass "/Game/PureBP/Utilities/BP_Assets/BP_Tarpet_Crate.BP_Tarpet_Crate_C" (Math|Transform|MakeTransform "1100.656372,2190.466797,170.000000" "0, 0, 0" "1.000000,1.000000,1.000000") "Undefined" 0 0))

(event Custom|CustomEvent_1
  (Game|Player|SetViewTargetwithBlend (Game|GetPlayerController 0) (Variables|Default|GetPlayerCamera) 1.0 "VTBlend_Linear" 0.0 true)
  (Collision|SetCollisionEnabled (Variables|Default|GetMur) "QueryAndPhysics")
  (Utilities|FlowControl|Delay 1.0)
  (Default|CallUnCinematic (Variables|Default|GetAs%20BP%20GI)))

(event EventBeginPlay)

(event Collision|EventActorBeginOverlap
  (params (OtherActor :type Actor%20Object%20Reference)))

(event EventTick
  (params (DeltaSeconds :type Float%20%28single-precision%29)))

(fn ConstructionScript)