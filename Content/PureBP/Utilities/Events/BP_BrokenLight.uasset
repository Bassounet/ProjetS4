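; BP_BrokenLight is a trigger volume that makes the first-person character's light malfunction while the player is inside its Box.
; Entering marks the light non-functional, calls LightBroken on the character, then disables the light after a short delay.
; Leaving calls LightBroken again, then after the same delay restores the functional flag and enables the light.
; An IsBroken flag gates both overlap events.
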(event OnComponentBeginOverlap(Box)
  (params (OverlappedComponent :type Primitive%20Component%20Object%20Reference) (OtherActor :type Actor%20Object%20Reference) (OtherComp :type Primitive%20Component%20Object%20Reference) (OtherBodyIndex :type Integer) (bFromSweep :type Boolean) (SweepResult :type Hit%20Result%20Structure%20%28by%20ref%29))
  (bind _asfirst_person_character (Utilities|Casting|CastToFirstPersonCharacter OtherActor))
  (if (not (Variables|Default|GetisBroken?))
    (Variables|Default|SetisBroken? true)
    (Variables|/Game/PureBP/Player/FirstPersonCharacter.FirstPersonCharacter_C|SetisLightFunctional? _asfirst_person_character false)
    (Default|LightBroken _asfirst_person_character)
    (Utilities|FlowControl|Delay 1.5)
    (Default|DisableLight _asfirst_person_character)))

(event OnComponentEndOverlap(Box)
  (params (OverlappedComponent :type Primitive%20Component%20Object%20Reference) (OtherActor :type Actor%20Object%20Reference) (OtherComp :type Primitive%20Component%20Object%20Reference) (OtherBodyIndex :type Integer))
  (bind _asfirst_person_character (Utilities|Casting|CastToFirstPersonCharacter OtherActor))
  (if (Variables|Default|GetisBroken?)
    (Variables|Default|SetisBroken? false)
    (Default|LightBroken _asfirst_person_character)
    (Utilities|FlowControl|Delay 1.5)
    (Variables|/Game/PureBP/Player/FirstPersonCharacter.FirstPersonCharacter_C|SetisLightFunctional? _asfirst_person_character true)
    (Default|EnableLight _asfirst_person_character)))

(event EventBeginPlay)

(event Collision|EventActorBeginOverlap
  (params (OtherActor :type Actor%20Object%20Reference)))

(event EventTick
  (params (DeltaSeconds :type Float%20%28single-precision%29)))

(fn ConstructionScript)