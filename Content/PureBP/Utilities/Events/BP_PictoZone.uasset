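; BP_PictoZone is a trigger zone that shows an on-screen indication, made of a pictogram, a button image and text, while the player is inside.
; Each zone creates its own W_Indication widget and adds it to the viewport on BeginPlay.
; When a FirstPersonCharacter enters the box, the zone fills the widget from its brush and text variables and calls Appear.
; When the character leaves, it calls Desappear.
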(event OnComponentBeginOverlap(Box)
  (params (OverlappedComponent :type Primitive%20Component%20Object%20Reference) (OtherActor :type Actor%20Object%20Reference) (OtherComp :type Primitive%20Component%20Object%20Reference) (OtherBodyIndex :type Integer) (bFromSweep :type Boolean) (SweepResult :type Hit%20Result%20Structure%20%28by%20ref%29))
  (bind _ref_widget (Variables|Default|GetREF_Widget))
  (Utilities|Casting|CastToFirstPersonCharacter OtherActor)
  (Class|Image|SetBrush (Variables|/Game/PureBP/UI/BP/W_Indication.W_Indication_C|GetImageToDisplay _ref_widget) (Variables|Default|GetBrushPicto))
  (Class|Image|SetBrush (Variables|/Game/PureBP/UI/BP/W_Indication.W_Indication_C|GetButton _ref_widget) (Variables|Default|GetBrushBtn))
  (Rendering|Components|TextRender|SetText (Variables|/Game/PureBP/UI/BP/W_Indication.W_Indication_C|GetTextBlock_64 _ref_widget) (Variables|Default|GetTextToDisplay))
  (Default|Appear (Variables|Default|GetREF_Widget)))

(event OnComponentEndOverlap(Box)
  (params (OverlappedComponent :type Primitive%20Component%20Object%20Reference) (OtherActor :type Actor%20Object%20Reference) (OtherComp :type Primitive%20Component%20Object%20Reference) (OtherBodyIndex :type Integer))
  (Utilities|Casting|CastToFirstPersonCharacter OtherActor)
  (Default|Desappear (Variables|Default|GetREF_Widget)))

(event EventBeginPlay
  (bind _returnvalue (UserInterface|CreateWidget "/Game/PureBP/UI/BP/W_Indication.W_Indication_C"))
  (bind _output_get (Variables|Default|SetREF_Widget _returnvalue))
  (UserInterface|Viewport|AddtoViewport _output_get 0))

(fn ConstructionScript)