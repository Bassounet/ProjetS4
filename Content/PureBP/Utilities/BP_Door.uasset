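; Interactive door that swings away from or toward either side, with optional key lock, on-screen prompt and crosshair highlight.
; Front and Back overlaps set the player's side and range, selecting one of two opposite-yaw timelines that Interact plays or reverses.
; Running into Collision1 or Collision2 kicks a closed door open at 10x speed with camera shake.
; The Front overlap also binds the death-reset dispatcher, which reverses only the TimeToOpenDoor timeline.
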(event OnComponentBeginOverlap(Front)
  (params (OverlappedComponent :type Primitive%20Component%20Object%20Reference) (OtherActor :type Actor%20Object%20Reference) (OtherComp :type Primitive%20Component%20Object%20Reference) (OtherBodyIndex :type Integer) (bFromSweep :type Boolean) (SweepResult :type Hit%20Result%20Structure%20%28by%20ref%29))
  ;[1 1 1] DETECT
  (Utilities|Casting|CastToBoxComponent OtherComp
    (:CastFailed
      (bind _asfirst_person_character (Utilities|Casting|CastToFirstPersonCharacter OtherActor))
      (Variables|REF|SetREF_FP _asfirst_person_character)
      (CallFunction|WichHUD)
      (Variables|Default|SetInRangeForOpen true)
      (Variables|Default|SetBack/Front "NewEnumerator0")
      (bind _asbp_gi (CallFunction|RecupDispatcherDie))
      (EventDispatchers|BindEventtoResetAfterDie _asbp_gi (delegate Custom|CloseDoor)))))

(event OnComponentBeginOverlap(Back)
  (params (OverlappedComponent :type Primitive%20Component%20Object%20Reference) (OtherActor :type Actor%20Object%20Reference) (OtherComp :type Primitive%20Component%20Object%20Reference) (OtherBodyIndex :type Integer) (bFromSweep :type Boolean) (SweepResult :type Hit%20Result%20Structure%20%28by%20ref%29))
  ;[1 1 1] Interaction Porte Arrière
  (Utilities|Casting|CastToBoxComponent OtherComp
    (:CastFailed
      (Utilities|Casting|CastToFirstPersonCharacter OtherActor)
      (CallFunction|WichHUD)
      (Variables|Default|SetInRangeForOpen true)
      (Variables|Default|SetBack/Front "NewEnumerator1"))))

(event OnComponentEndOverlap(Front)
  (params (OverlappedComponent :type Primitive%20Component%20Object%20Reference) (OtherActor :type Actor%20Object%20Reference) (OtherComp :type Primitive%20Component%20Object%20Reference) (OtherBodyIndex :type Integer))
  ;[1 1 1] DETECT
  (Utilities|Casting|CastToBoxComponent OtherComp
    (:CastFailed
      (Utilities|Casting|CastToFirstPersonCharacter OtherActor)
      (Variables|Default|SetInRangeForOpen false)
      (bind _asbp_gi (CallFunction|RecupDispatcherDie))
      (EventDispatchers|UnbindallEventsfromResetAfterDie _asbp_gi)
      (CallFunction|HUDDoorOFF))))

(event OnComponentEndOverlap(Back)
  (params (OverlappedComponent :type Primitive%20Component%20Object%20Reference) (OtherActor :type Actor%20Object%20Reference) (OtherComp :type Primitive%20Component%20Object%20Reference) (OtherBodyIndex :type Integer))
  ;[1 1 1] Interaction Porte Arrière
  (Utilities|Casting|CastToBoxComponent OtherComp
    (:CastFailed
      (Utilities|Casting|CastToFirstPersonCharacter OtherActor)
      (CallFunction|HUDDoorOFF)
      (Variables|Default|SetInRangeForOpen false))))

(event OnComponentBeginOverlap(Collision1)
  (params (OverlappedComponent :type Primitive%20Component%20Object%20Reference) (OtherActor :type Actor%20Object%20Reference) (OtherComp :type Primitive%20Component%20Object%20Reference) (OtherBodyIndex :type Integer) (bFromSweep :type Boolean) (SweepResult :type Hit%20Result%20Structure%20%28by%20ref%29))
  ;[1 1 1] DETECT
  (Utilities|Casting|CastToBoxComponent OtherComp
    (:CastFailed
      (bind _asfirst_person_character (Utilities|Casting|CastToFirstPersonCharacter OtherActor))
      (Variables|Default|SetInRangeForOpen true)
      (if (Variables|/Game/FirstPerson/FirstPersonBP/Blueprints/FirstPersonCharacter.FirstPersonCharacter_C|GetIsRunning _asfirst_person_character)
        (switch Utilities|FlowControl|Switch|SwitchonEN_ModeOpenDoor (Variables|Default|GetModeOpened)
          (:NewEnumerator0
            (CallFunction|KickDoor)))))))

(event OnComponentBeginOverlap(Collision2)
  (params (OverlappedComponent :type Primitive%20Component%20Object%20Reference) (OtherActor :type Actor%20Object%20Reference) (OtherComp :type Primitive%20Component%20Object%20Reference) (OtherBodyIndex :type Integer) (bFromSweep :type Boolean) (SweepResult :type Hit%20Result%20Structure%20%28by%20ref%29))
  ;[1 1 1] Interaction Porte Arrière
  (Utilities|Casting|CastToBoxComponent OtherComp
    (:CastFailed
      (bind _asfirst_person_character (Utilities|Casting|CastToFirstPersonCharacter OtherActor))
      (Variables|Default|SetInRangeForOpen true)
      (if (Variables|/Game/FirstPerson/FirstPersonBP/Blueprints/FirstPersonCharacter.FirstPersonCharacter_C|GetIsRunning _asfirst_person_character)
        (switch Utilities|FlowControl|Switch|SwitchonEN_ModeOpenDoor (Variables|Default|GetModeOpened)
          (:NewEnumerator0
            (CallFunction|KickDoor)))))))

(event Custom|CloseDoor
  ;[1 1 1] DETECT
  (CallFunction|ResetAfterDie))

(event Custom|KickDoor
  ;[1 1 1] Open It
  (if (not (Variables|Default|GetKey?))
    (Components|Timeline|SetPlayRate (Variables|Default|GetTimeToOpenDoor) 1e+01 :!label _label)
    (CallFunction|CamShakeLight)
    (switch Utilities|FlowControl|Switch|SwitchonEN_PosFromDoor (Variables|Default|GetBack/Front)
      (:NewEnumerator0
        (switch Utilities|FlowControl|Switch|SwitchonEN_ModeOpenDoor (Variables|Default|GetModeOpened)
          (:NewEnumerator0
            (bind _openthedoor (Timeline|TimeToOpenDoor Play)
              (:Update
                (Transformation|SetRelativeRotation (Variables|Default|GetStaticMesh) (Math|Rotator|MakeRotator 0.0 0.0 (Math|Float|Lerp 0.0 -9e+01 _openthedoor)) false false))
              (:Finished
                (switch Utilities|FlowControl|Switch|SwitchonEN_ModeOpenDoor (Variables|Default|GetModeOpened)
                  (:NewEnumerator0
                    (Variables|Default|SetModeOpened "NewEnumerator1"))
                  (:NewEnumerator1
                    (Variables|Default|SetModeOpened "NewEnumerator0"))))))
          (:NewEnumerator1
            (Timeline|TimeToOpenDoor Reverse))
          (:NewEnumerator2
            (bind _openthedoor_2 (Timeline|Timeline_1 Reverse)
              (:Update
                (Transformation|SetRelativeRotation (Variables|Default|GetStaticMesh) (Math|Rotator|MakeRotator 0.0 0.0 (Math|Float|Lerp 0.0 9e+01 _openthedoor_2)) false false))
              (:Finished
                (switch Utilities|FlowControl|Switch|SwitchonEN_ModeOpenDoor (Variables|Default|GetModeOpened)
                  (:NewEnumerator0
                    (Variables|Default|SetModeOpened "NewEnumerator2"))
                  (:NewEnumerator2
                    (Variables|Default|SetModeOpened "NewEnumerator0"))))))))
      (:NewEnumerator1
        (switch Utilities|FlowControl|Switch|SwitchonEN_ModeOpenDoor (Variables|Default|GetModeOpened)
          (:NewEnumerator0
            (Timeline|Timeline_1 Play))
          (:NewEnumerator1
            (Timeline|TimeToOpenDoor Reverse))
          (:NewEnumerator2
            (Timeline|Timeline_1 Reverse)))))
    (elif (Variables|/Game/FirstPerson/FirstPersonBP/Blueprints/FirstPersonCharacter.FirstPersonCharacter_C|GetGotKey? (Variables|REF|GetREF_FP))
      (goto _label))))

(event Custom|ResetAfterDie
  ;[1 1 1] Open It
  (bind _openthedoor (Timeline|TimeToOpenDoor Reverse)
    (:Update
      (Transformation|SetRelativeRotation (Variables|Default|GetStaticMesh) (Math|Rotator|MakeRotator 0.0 0.0 (Math|Float|Lerp 0.0 -9e+01 _openthedoor)) false false))
    (:Finished
      (switch Utilities|FlowControl|Switch|SwitchonEN_ModeOpenDoor (Variables|Default|GetModeOpened)
        (:NewEnumerator0
          (Variables|Default|SetModeOpened "NewEnumerator1"))
        (:NewEnumerator1
          (Variables|Default|SetModeOpened "NewEnumerator0"))))))

(event Custom|DoorActivate
  ;[1 1 1] Open It
  (Components|Timeline|SetPlayRate (Variables|Default|GetTimeToOpenDoor) 1.0)
  (if (Variables|Default|GetInRangeForOpen)
    (switch Utilities|FlowControl|Switch|SwitchonEN_PosFromDoor (Variables|Default|GetBack/Front)
      (:NewEnumerator0
        (switch Utilities|FlowControl|Switch|SwitchonEN_ModeOpenDoor (Variables|Default|GetModeOpened)
          (:NewEnumerator0
            (bind _openthedoor (Timeline|TimeToOpenDoor Play)
              (:Update
                (Transformation|SetRelativeRotation (Variables|Default|GetStaticMesh) (Math|Rotator|MakeRotator 0.0 0.0 (Math|Float|Lerp 0.0 -9e+01 _openthedoor)) false false))
              (:Finished
                (switch Utilities|FlowControl|Switch|SwitchonEN_ModeOpenDoor (Variables|Default|GetModeOpened)
                  (:NewEnumerator0
                    (Variables|Default|SetModeOpened "NewEnumerator1"))
                  (:NewEnumerator1
                    (Variables|Default|SetModeOpened "NewEnumerator0"))))))
          (:NewEnumerator1
            (Timeline|TimeToOpenDoor Reverse))
          (:NewEnumerator2
            (bind _openthedoor_2 (Timeline|Timeline_1 Reverse)
              (:Update
                (Transformation|SetRelativeRotation (Variables|Default|GetStaticMesh) (Math|Rotator|MakeRotator 0.0 0.0 (Math|Float|Lerp 0.0 9e+01 _openthedoor_2)) false false))
              (:Finished
                (switch Utilities|FlowControl|Switch|SwitchonEN_ModeOpenDoor (Variables|Default|GetModeOpened)
                  (:NewEnumerator0
                    (Variables|Default|SetModeOpened "NewEnumerator2"))
                  (:NewEnumerator2
                    (Variables|Default|SetModeOpened "NewEnumerator0"))))))))
      (:NewEnumerator1
        (switch Utilities|FlowControl|Switch|SwitchonEN_ModeOpenDoor (Variables|Default|GetModeOpened)
          (:NewEnumerator0
            (Timeline|Timeline_1 Play))
          (:NewEnumerator1
            (Timeline|TimeToOpenDoor Reverse))
          (:NewEnumerator2
            (Timeline|Timeline_1 Reverse)))))))

(event Custom|HUDDoorOFF
  ;[1 1 1] HUD Gest
  (Widget|SetVisibility (Variables|REF|GetREF_WidgetDoorOpen) "Hidden"))

(event Custom|HUD_OpenDoor
  (bind _ref_widgetdooropen (Variables|REF|GetREF_WidgetDoorOpen))
  (bind _ref_widgetdooropen_2 (Variables|REF|GetREF_WidgetDoorOpen))
  ;[1 1 1] HUD Gest
  (if (not (Variables|Default|GetKey?))
    (Widget|SetVisibility _ref_widgetdooropen_2 "Visible" :!label _label)
    (Rendering|Components|TextRender|SetText (Variables|/Game/PureBP/UI/W_DoorInteract.W_DoorInteract_C|GetTextBlock_0 _ref_widgetdooropen_2) "[F] To open door")
    (elif (Variables|/Game/FirstPerson/FirstPersonBP/Blueprints/FirstPersonCharacter.FirstPersonCharacter_C|GetGotKey? (Variables|REF|GetREF_FP))
      (goto _label)
      (else
        (Widget|SetVisibility _ref_widgetdooropen "Visible")
        (Rendering|Components|TextRender|SetText (Variables|/Game/PureBP/UI/W_DoorInteract.W_DoorInteract_C|GetTextBlock_0 _ref_widgetdooropen) "Vous avez besoin de la clef")))))

(event Custom|HUDCloseDoor
  (bind _ref_widgetdooropen (Variables|REF|GetREF_WidgetDoorOpen))
  ;[1 1 1] HUD Gest
  (Widget|SetVisibility _ref_widgetdooropen "Visible")
  (Rendering|Components|TextRender|SetText (Variables|/Game/PureBP/UI/W_DoorInteract.W_DoorInteract_C|GetTextBlock_0 _ref_widgetdooropen) "[F] To close door"))

(event Custom|WichHUD
  ;[1 1 1] Select HUD
  (switch Utilities|FlowControl|Switch|SwitchonEN_ModeOpenDoor (Variables|Default|GetModeOpened)
    (:NewEnumerator0
      (CallFunction|HUDOpenDoor))
    (:NewEnumerator1
      (CallFunction|HUDCloseDoor))
    (:NewEnumerator2
      (CallFunction|HUDCloseDoor))))

(event EventBeginPlay
  ;[1 1 1] GetSomeRef
  (bind _returnvalue (UserInterface|CreateWidget "/Game/PureBP/UI/W_DoorInteract.W_DoorInteract_C"))
  (Variables|REF|SetREF_WidgetDoorOpen _returnvalue)
  (UserInterface|Viewport|AddtoViewport (Variables|REF|GetREF_WidgetDoorOpen) 0)
  (Widget|SetVisibility (Variables|REF|GetREF_WidgetDoorOpen) "Hidden"))

(event EventInteract
  ;[1 1 1] Interaction
  (if (not (Variables|Default|GetKey?))
    (CallFunction|DoorActivate)
    (elif (Variables|/Game/FirstPerson/FirstPersonBP/Blueprints/FirstPersonCharacter.FirstPersonCharacter_C|GetGotKey? (Variables|REF|GetREF_FP))
      (CallFunction|DoorActivate))))

(event EventCursored
  ;[1 1 1] Cursor Interaction
  (bind _ref_mainhud (CallFunction|GetHUD))
  (Appearance|SetColorandOpacity (Variables|/Game/PureBP/UI/W_MainHud.W_MainHud_C|GetPrincipalCursor _ref_mainhud) "(R=1.000000,G=0.000000,B=0.000000,A=1.000000)" :!class /Script/UMG.Image))

(event EventUnCursored
  ;[1 1 1] Cursor Interaction
  (Appearance|SetColorandOpacity (Variables|/Game/PureBP/UI/W_MainHud.W_MainHud_C|GetPrincipalCursor (stale EventCursored _ref_mainhud)) "(R=1.000000,G=1.000000,B=1.000000,A=1.000000)" :!class /Script/UMG.Image))

(fn ConstructionScript)