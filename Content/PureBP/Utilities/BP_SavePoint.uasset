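; BP_SavePoint is a save point actor that stores a respawn location on the first-person character.
; A box overlap caches the FirstPersonCharacter and toggles RangeToSave, though Interact never checks that flag.
; Interact copies the root's world location into ZoneRespawnLocation without writing a save game.
; It then briefly shows that location on its own W_MainHud, created at BeginPlay, with a blur fade before hiding the widget.
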(event OnComponentBeginOverlap(Box)
  (params (OverlappedComponent :type Primitive%20Component%20Object%20Reference) (OtherActor :type Actor%20Object%20Reference) (OtherComp :type Primitive%20Component%20Object%20Reference) (OtherBodyIndex :type Integer) (bFromSweep :type Boolean) (SweepResult :type Hit%20Result%20Structure%20%28by%20ref%29))
  ;[1 1 1] Interact in/ Out
  (bind _asfirst_person_character (Utilities|Casting|CastToFirstPersonCharacter OtherActor))
  (Variables|Default|SetREF_Fp _asfirst_person_character)
  (Variables|Default|SetRangeToSave? true))

(event OnComponentEndOverlap(Box)
  (params (OverlappedComponent :type Primitive%20Component%20Object%20Reference) (OtherActor :type Actor%20Object%20Reference) (OtherComp :type Primitive%20Component%20Object%20Reference) (OtherBodyIndex :type Integer))
  ;[1 1 1] Interact in/ Out
  (Utilities|Casting|CastToFirstPersonCharacter OtherActor)
  (Variables|Default|SetRangeToSave? false))

(event EventInteract
  (bind _ref_mainhud (Variables|Default|GetREF_MainHud))
  ;[1 1 1] Save
  (bind _output_get (Variables|/Game/FirstPerson/FirstPersonBP/Blueprints/FirstPersonCharacter.FirstPersonCharacter_C|SetZone%20Respawn%20Location (Variables|Default|GetREF_Fp) (Transformation|GetWorldLocation (Variables|Default|GetDefaultSceneRoot))))
  (Widget|SetVisibility (Variables|/Game/PureBP/UI/W_MainHud.W_MainHud_C|GetSave _ref_mainhud) "Visible")
  (Default|FadeBlurin _ref_mainhud)
  (Rendering|Components|TextRender|SetText (Variables|/Game/PureBP/UI/W_MainHud.W_MainHud_C|GetZoneTextBlur _ref_mainhud) (Utilities|Text|ToText(String) _output_get))
  (Utilities|FlowControl|Delay 2.0)
  (Default|FadeBlurOut _ref_mainhud)
  (Widget|SetVisibility _ref_mainhud "Hidden"))

(event EventBeginPlay
  (bind _returnvalue (UserInterface|CreateWidget "/Game/PureBP/UI/W_MainHud.W_MainHud_C"))
  (bind _output_get (Variables|Default|SetREF_MainHud _returnvalue))
  (UserInterface|Viewport|AddtoViewport _output_get 0))

(fn ConstructionScript)